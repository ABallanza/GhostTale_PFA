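; PDA_Effects is an effect asset for possessed objects, holding identity, fear type and VFX data exposed through getters.
; ActivateEffect casts its stored owner to BP_PossessedObject and, for the Morphing type, attaches a buff VFX to the body and swaps its static mesh.
; DestroyVFX removes that VFX, while ApplicateEffect only prints debug text.
; The calls that would frighten the Adventurer are disconnected, so activation applies no fear.
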(event Custom|Applicate%20Effect
  (params (Objet :type Name))
  (Development|PrintText 0 (Utilities|Text|FormatText "Je suis attaché à {Objet} et je suis {Effect}" Objet (Variables|Identity|GetName)) true true "(R=1.000000,G=0.023483,B=0.724213,A=1.000000)" 1e+01))

(event Custom|Activate%20Effect
  (params (Adventurer :type BP%20Adventurer%20Class%20Object%20Reference) (Fear%20Amount :type Float%20%28double-precision%29))
  (bind _asbp_possessed_object (Utilities|Casting|CastToBP_PossessedObject (Variables|Default|GetOwner)))
  (switch Utilities|FlowControl|Switch|SwitchonE_EffectType (Variables|Default|GetEffect%20type)
    (:NewEnumerator2
      (bind _returnvalue (Niagara|SpawnSystemAttached "/Game/GA/VFX/NiagaraSystem/Magic_Buff_Orange.Magic_Buff_Orange" (Default|GetBody _asbp_possessed_object) "None" (Transformation|GetWorldLocation (Default|GetBody _asbp_possessed_object)) (Transformation|GetWorldRotation (Default|GetBody _asbp_possessed_object)) "KeepWorldPosition" false))
      (Variables|Default|SetCurrent%20VFX _returnvalue)
      (Components|StaticMesh|SetStaticMesh (Default|GetBody _asbp_possessed_object) (Variables|Default|GetNew%20Mesh)))))

(event Custom|Destroy%20VFX
  (Components|DestroyComponent (Variables|Default|GetCurrent%20VFX)))

(fn SetOwner
  (params (Owner :type Actor%20Object%20Reference))
  (Variables|Default|SetOwner Owner))

(fn GetFearType
  (return (Variables|Effet|GetFearType)))

(fn GetFearVFX
  (return (Variables|Effect|GetVFX%20Correspondance)))

(fn GetIdentity
  (return (Variables|Identity|GetName) (Variables|Identité|GetDescription) (Variables|Identité|GetIcone)))