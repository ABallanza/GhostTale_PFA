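; Utility Blueprint for a generic gauge that fills or empties within zero and MaxGauge and is divided into discrete steps.
; BeginPlay builds evenly spaced step thresholds; ChangeGauge applies a clamped signed amount, then recounts the reached step.
; Getters expose value, percent, step and status.
; Timed changes are unimplemented, so all apply instantly, and SetStatus only ever sets IsFull false, leaving its IsEmpty writes unreachable.
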(event Custom|ChangeGauge
  (params (Length :type Float%20%28double-precision%29) (IsNegative :type Boolean) (Amount :type Float%20%28double-precision%29))
  ;[0.03646 0.6961 1 0.5] Fonction principale pour modifier la jauge
  ; Lentgh = temps que la bar met à se remplire ou se vider (pas encore dev, mettre à 0 pour que ce soit instantané)
  ; Is Negative = La bar se vide si true
  ; Amount = Le montant du changement
  ;;[0 0.1671 1 0.8] Calcule la nouvelle valeur de la jauge
  (bind (_instant _newgauge) (CallFunction|UpdateGauge Length IsNegative Amount))
  ;;[0.2119 0 1 1 10] Vérifie si la jauge dois se modifie immédiatement ou sur la durée
  (if _instant
    _
    (else
      _))
  (Variables|Default|SetCurrentGauge _newgauge)
  (bind _current_level (CallFunction|UpdateGaugeLevel))
  (Variables|Default|SetCurrent%20Step _current_level)
  (CallFunction|SetStatus))

(event EventBeginPlay
  ;[1 1 1] Met à jour certaines variables en fonction des paramètres pré-enregistrés
  (CallFunction|SetStatus)
  (CallFunction|SetGaugeSteps))

(fn GetStatus
  (return (Variables|Default|GetIsFull) (Variables|Default|GetIsEmpty) (Variables|Default|GetMaxGauge) (Variables|Default|GetCurrentGauge)))

(fn SetStatus
  (bind _currentgauge (Variables|Default|GetCurrentGauge))
  (if (== _currentgauge 0)
    (Variables|Default|SetIsFull false)
    (elif (== _currentgauge (Variables|Default|GetMaxGauge))
      (Variables|Default|SetIsFull false)
      (else
        (Variables|Default|SetIsFull false)))))

(fn UpdateGauge
  (params (Length :type Float%20%28double-precision%29) (IsNegative :type Boolean) (Amount :type Float%20%28double-precision%29))
  (if (== Length 0.0)
    (LocalVariables|SetIsInstant true)
    (else
      (LocalVariables|SetIsInstant false)))
  (if IsNegative
    (LocalVariables|SetTrueAmount (* Amount -1.0))
    (else
      (LocalVariables|SetTrueAmount Amount)))
  (if (> (+ (LocalVariables|GetTrueAmount) (Variables|Default|GetCurrentGauge)) (Variables|Default|GetMaxGauge))
    (return (LocalVariables|GetIsInstant) (Variables|Default|GetMaxGauge))
    (elif (< (+ (LocalVariables|GetTrueAmount) (Variables|Default|GetCurrentGauge)) 0.0)
      (return (LocalVariables|GetIsInstant) 0.0)
      (else
        (return (LocalVariables|GetIsInstant) (+ (LocalVariables|GetTrueAmount) (Variables|Default|GetCurrentGauge)))))))

(fn GetGaugePercent
  (return (/ (Variables|Default|GetCurrentGauge) (Variables|Default|GetMaxGauge))))

(fn GetMaxGauge
  (return (Variables|Default|GetMaxGauge)))

(fn GetCurrentGauge
  (return (Variables|Default|GetCurrentGauge)))

(fn GetIsFull
  (return (Variables|Default|GetIsFull)))

(fn GetIsEmpty
  (return (Variables|Default|GetIsEmpty)))

(fn GetMaxStep
  (return (Variables|Default|GetMax%20Step)))

(fn GetCurrentStep
  (return (Variables|Default|GetCurrent%20Step)))

(fn SetGaugeSteps
  (LocalVariables|SetLevel%20Step (/ (Variables|Default|GetMaxGauge) (Variables|Default|GetMax%20Step)))
  (for _index (range 1 (Variables|Default|GetMax%20Step))
    (Utilities|Array|Add (Variables|Default|GetGaugeLevelSteps) (* _index (LocalVariables|GetLevel%20Step)))))

(fn UpdateGaugeLevel
  (for _index (range 0 (- (Variables|Default|GetMax%20Step) 1))
    (if (<= (Utilities|Array|Get(acopy) (Variables|Default|GetGaugeLevelSteps) _index) (Variables|Default|GetCurrentGauge))
      (Math|Integer|IncrementInt (LocalVariables|GetLevelCounter))))
  (return (LocalVariables|GetLevelCounter)))