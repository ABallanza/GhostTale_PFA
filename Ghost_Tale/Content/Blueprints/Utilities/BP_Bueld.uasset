(event Custom|ResetBuildMode
  ;[0 1 0.4408] Raycast for affichage
  (Utilities|Array|Clear (Variables|Default|GetIgnoredElement))
  (bind _preview_mesh (Variables|Components|GetPreview%20Mesh)
    (:then
      (Components|StaticMesh|SetStaticMesh _preview_mesh 0)
      (Variables|Components|SetPreview%20Mesh 0)
      (Utilities|FlowControl|DoOnce false) ; enters at Reset
    )
    (:else)))

(event Custom|Destroy%20Mode
  (bind _returnvalue (Game|GetPlayerController 0))
  (bind (_worldlocation _worlddirection) (Game|Player|ConvertMouseLocationToWorldSpace _returnvalue))
  ;[1 0.02677 0 0.456] Destroy Trap
  (bind (_outhit _returnvalue_2) (Collision|LineTraceByChannel _worldlocation (+ _worldlocation (* _worlddirection 5e+03)) "TraceTypeQuery1" false 0 "None"))
  (if _returnvalue_2
    (bind _asbp_corridor (Utilities|Casting|CastToBP_corridor (.HitActor (Collision|BreakHitResult _outhit)))
      (:then
        (Utilities|Array|Add (Variables|Default|GetChangedCorridor) _asbp_corridor)
        (Transformation|SetRelativeLocation (Variables|/Game/Blueprints/LevelElements/BP_corridor.BP_corridor_C|GetBox _asbp_corridor) (Math|Vector|MakeVector (.x (Variables|/Script/Engine.SceneComponent|GetRelativeLocation (Variables|/Game/Blueprints/LevelElements/BP_corridor.BP_corridor_C|GetBox _asbp_corridor))) (.y (Variables|/Script/Engine.SceneComponent|GetRelativeLocation (Variables|/Game/Blueprints/LevelElements/BP_corridor.BP_corridor_C|GetBox _asbp_corridor))) (+ (.z (Variables|/Script/Engine.SceneComponent|GetRelativeLocation (Variables|/Game/Blueprints/LevelElements/BP_corridor.BP_corridor_C|GetBox _asbp_corridor))) -2e+03)) false false))
      (:CastFailed
        (Utilities|Casting|CastToBP_BuildMaster (.HitActor (Collision|BreakHitResult _outhit))
          (:then
            (CallFunction|TrapOverlaped (.HitComponent (Collision|BreakHitResult _outhit)) (.HitActor (Collision|BreakHitResult _outhit))))
          (:CastFailed
            (CallFunction|DoNotTouch)))))
    (else
      (CallFunction|DoNotTouch))))

(event Custom|MWD
  ;[0 0.54 1] Mouse Wheel event
  (if (< (+ (Variables|Default|GetTowerIndex) -1) 0)
    (Variables|Default|SetTowerIndex (+ (Utilities|Array|Length (Variables|Default|GetDT_trap)) -1))
    (else
      (Variables|Default|SetTowerIndex (+ (Variables|Default|GetTowerIndex) -1))))
  (Default|OnWheelEvent (Variables|/Game/Blueprints/GUI/WBP_Main.WBP_Main_C|GetWB_TrapBook (Variables|Default|GetMain%20Widget)) (Variables|Default|GetTowerIndex))
  (Variables|Default|SetBuildMode true)
  (CallFunction|ResetBuildMode))

(event Custom|MWU
  ;[0 0.54 1] Mouse Wheel event
  (if (> (+ (Variables|Default|GetTowerIndex) 1) (+ (Utilities|Array|Length (Variables|Default|GetDT_trap)) -1))
    (Variables|Default|SetTowerIndex 0)
    (else
      (Variables|Default|SetTowerIndex (+ (Variables|Default|GetTowerIndex) 1))))
  (Default|OnWheelEvent (Variables|/Game/Blueprints/GUI/WBP_Main.WBP_Main_C|GetWB_TrapBook (Variables|Default|GetMain%20Widget)) (Variables|Default|GetTowerIndex))
  (Variables|Default|SetBuildMode true)
  (CallFunction|ResetBuildMode))

(event Custom|TrapOverlaped
  (params (Target :type Primitive%20Component%20Object%20Reference) (Actor :type Actor%20Object%20Reference))
  ;[1 0.02677 0 0.456] Destroy Trap
  (if (not (Variables|Default|GetDestroyMode))
    (for _array_element (Components|GetChildrenComponents (Transformation|GetAttachParent Target) false)
      (bind _asprimitive_component (Utilities|Casting|CastToPrimitiveComponent _array_element))
      (Utilities|Array|Add (Variables|Default|GetComponentList) _asprimitive_component))
    (CallFunction|DestroyTowerPreview Actor (Variables|Default|GetComponentList))
    (Utilities|Array|Clear (Variables|Default|GetComponentList))))

(event Custom|Enable%20BP%20Trap
  (bind _self self)
  (bind _main_widget (Variables|Default|GetMain%20Widget))
  (bind _wb_trapbook (Variables|/Game/Blueprints/GUI/WBP_Main.WBP_Main_C|GetWB_TrapBook _main_widget))
  (Components|Tick|SetComponentTickEnabled _self true)
  (Components|Activation|SetActive _self true false)
  (Widget|SetIsEnabled _wb_trapbook true)
  (Widget|SetVisibility _wb_trapbook "Visible"))

(event Custom|do%20not%20touch
  ;[1 0.02677 0 0.456] Destroy Trap
  (if (Variables|Default|GetDestroyMode)
    (Variables|Default|SetDestroyMode false)
    (Utilities|IsValid (Utilities|Array|Get(acopy) (Variables|Default|GetD_Component))
      (:Is%20Valid
        (for _array_element (Variables|Default|GetD_Component)
          (Rendering|Material|SetMaterial _array_element 0 (Variables|Default|GetD_Component_OriginalMaterial))
          (Default|Add/RemoveMappingContext (.AsBP%20Camera%20Controller (Utilities|Casting|CastToBP_CameraController (Game|GetPlayerController 0))) true "/Game/Blueprints/Controls/IMC_TrapMode.IMC_TrapMode"))))))

(event Custom|AffichageRayCast
  (params (Actor%20to%20Ignore :type Array%20of%20Actor%20Object%20References))
  (bind _returnvalue (Game|GetPlayerController 0))
  (bind (_worldlocation _worlddirection) (Game|Player|ConvertMouseLocationToWorldSpace _returnvalue))
  ;[0 1 0.4408] Raycast for affichage
  (bind (_outhit _returnvalue_2) (Collision|LineTraceByChannel _worldlocation (+ _worldlocation (* _worlddirection 5e+03)) "TraceTypeQuery3" false Actor%20to%20Ignore "None" true "(R=1.000000,G=0.000000,B=0.056582,A=1.000000)" "(R=0.000000,G=1.000000,B=0.000000,A=1.000000)" 1e+01))
  (if _returnvalue_2
    (bind _asbp_corridor (Utilities|Casting|CastToBP_corridor (.HitActor (Collision|BreakHitResult _outhit)))
      (:then
        (Utilities|Array|Add (Variables|Default|GetIgnoredElement) _asbp_corridor)
        (CallFunction|AffichageRayCast (Variables|Default|GetIgnoredElement)))
      (:CastFailed
        (Utilities|FlowControl|Sequence
          (:then_0
            (Utilities|FlowControl|DoOnce false
              (:Completed
                (bind _returnvalue_3 (Game|AddComponentbyClass (.AsActor (Utilities|Casting|CastToActor (Variables|Default|GetPlayer))) "/Script/Engine.StaticMeshComponent" false (Variables|Default|GetBuild%20Preview%20Transform)))
                (bind _output_get (Variables|Components|SetPreview%20Mesh _returnvalue_3))
                (Components|StaticMesh|SetStaticMesh _output_get (.Mesh (Utilities|Struct|BreakST_TrapType (Utilities|Array|Get(acopy) (Variables|Default|GetDT_trap) (Variables|Default|GetTowerIndex)))))
                (Collision|SetCollisionEnabled (Variables|Components|GetPreview%20Mesh) "NoCollision")
                (if (and (Variables|Default|GetBuildable) (> (Variables|/Game/Blueprints/GUI/WB_TrapBook.WB_TrapBook_C|GetChildrenCount (Variables|/Game/Blueprints/GUI/WBP_Main.WBP_Main_C|GetWB_TrapBook (Variables|Default|GetMain%20Widget))) 0))
                  (Rendering|Material|SetMaterial (Variables|Components|GetPreview%20Mesh) 0 "/Game/Blueprints/Interactibles/Tower/Visual/MI_TowerPreview.MI_TowerPreview")
                  (else
                    (Rendering|Material|SetMaterial (Variables|Components|GetPreview%20Mesh) 0 "/Game/Blueprints/Interactibles/Tower/Visual/MI_TowerDestroy.MI_TowerDestroy"))))))
          (:then_1
            (if (Variables|Default|GetBuildable)
              (Variables|Default|SetBuild%20Preview%20Transform (Transformation|GetWorldTransform (Variables|/Game/Blueprints/LevelElements/BP_corridor.BP_corridor_C|GetTrapoint (Variables|Default|GetTargetedCorridor))))
              (else
                (Variables|Default|SetBuild%20Preview%20Transform (Math|Transform|MakeTransform (.ImpactPoint (Collision|BreakHitResult _outhit)) "0, 0, 0" "1.000000,1.000000,1.000000"))))
            (Transformation|SetWorldTransform (Variables|Components|GetPreview%20Mesh) (Variables|Default|GetBuild%20Preview%20Transform) false false)))))))

(event Custom|ManualSwitch
  (params (index :type Integer))
  ;[0 0.54 1] Mouse Wheel event
  (Variables|Default|SetTowerIndex index)
  (for _array_element (Variables|Default|GetChangedCorridor)
    (Utilities|IsValid _array_element
      (:Is%20Valid
        (Default|ResetHitboxSize _array_element))))
  (Utilities|Array|Clear (Variables|Default|GetChangedCorridor))
  (Variables|Default|SetNewTrapSelected true)
  (Variables|Default|SetBuildMode true)
  (CallFunction|ResetBuildMode))

(event Custom|DestroyTowerPreview
  (params (Actor :type Actor%20Object%20Reference) (Component :type Array%20of%20Primitive%20Component%20Object%20References))
  ;[1 0.02677 0 0.456] Destroy Trap
  ;;[1 0.4087 0] Change material
  (Variables|Default|SetD_Actor Actor)
  (Variables|Default|SetD_Component Component)
  (Variables|Default|SetDestroyMode true)
  (Default|Add/RemoveMappingContext (.AsBP%20Camera%20Controller (Utilities|Casting|CastToBP_CameraController (Game|GetPlayerController 0))) false "/Game/Blueprints/Controls/IMC_TrapMode.IMC_TrapMode")
  (for _array_element (Variables|Default|GetD_Component)
    (Variables|Default|SetD_Component_OriginalMaterial (Rendering|Material|GetMaterial _array_element 0))
    (Rendering|Material|SetMaterial _array_element 0 "/Game/Blueprints/Interactibles/Tower/Visual/MI_TowerDestroy.MI_TowerDestroy")))

(event Custom|PreviewLook
  (bind _returnvalue (Game|GetPlayerController 0))
  (bind (_worldlocation _worlddirection) (Game|Player|ConvertMouseLocationToWorldSpace _returnvalue))
  ;[0 1 0.07869] Raycast for detection
  (bind (_outhit _returnvalue_2) (Collision|LineTraceByChannel _worldlocation (+ _worldlocation (* _worlddirection 5e+03)) "TraceTypeQuery1" false 0 "None" true "(R=0.848955,G=0.000000,B=1.000000,A=1.000000)"))
  (if _returnvalue_2
    (bind _asbp_corridor (Utilities|Casting|CastToBP_corridor (.HitActor (Collision|BreakHitResult _outhit)))
      (:then
        (Utilities|Array|Add (Variables|Default|GetIgnoredElement) _asbp_corridor)
        (if (Variables|/Game/Blueprints/LevelElements/BP_corridor.BP_corridor_C|GetHaveTrap _asbp_corridor)
          (if (Variables|Default|GetBuildable) :!label _label
            (CallFunction|ResetBuildMode))
          (Variables|Default|SetBuildable false)
          (else
            (Variables|Default|SetTargetedCorridor _asbp_corridor)
            (if (Variables|Default|GetBuildable)
              _
              (else
                (CallFunction|ResetBuildMode)))
            (Variables|Default|SetBuildable true))))
      (:CastFailed
        (goto _label)))
    (CallFunction|AffichageRayCast (Variables|Default|GetIgnoredElement))))

(event Custom|Get%20Widget%20Ref
  (params (Widget%20Ref :type WBP%20Main%20Object%20Reference))
  (Variables|Default|SetMain%20Widget Widget%20Ref))

(event Custom|MouseR%20click
  ;[0 0.03631 1] Enable-Disable buildmode
  (Variables|Default|SetBuildMode false)
  (Default|UnselectSlot (Variables|/Game/Blueprints/GUI/WBP_Main.WBP_Main_C|GetWB_TrapBook (Variables|Default|GetMain%20Widget)))
  ;[1 0 0.7789] reset everything
  (CallFunction|ResetBuildMode)
  (if (Variables|Default|GetDestroyMode)
    (Variables|Default|SetDestroyMode false)
    (Utilities|IsValid (Utilities|Array|Get(acopy) (Variables|Default|GetD_Component))
      (:Is%20Valid
        (for _array_element (Variables|Default|GetD_Component)
          (Rendering|Material|SetMaterial _array_element 0 (Variables|Default|GetD_Component_OriginalMaterial))
          (Default|Add/RemoveMappingContext (.AsBP%20Camera%20Controller (Utilities|Casting|CastToBP_CameraController (Game|GetPlayerController 0))) true "/Game/Blueprints/Controls/IMC_TrapMode.IMC_TrapMode"))))))

(event Custom|Build
  ;[0 0.03631 1] Enable-Disable buildmode
  (if (not (Variables|Default|GetBuildMode))
    (for _array_element (Variables|Default|GetChangedCorridor)
      (Utilities|IsValid _array_element
        (:Is%20Valid
          (Default|ResetHitboxSize _array_element))))
    (Utilities|Array|Clear (Variables|Default|GetChangedCorridor))
    (Variables|Default|SetBuildMode true)
    (Default|OnWheelEvent (Variables|/Game/Blueprints/GUI/WBP_Main.WBP_Main_C|GetWB_TrapBook (Variables|Default|GetMain%20Widget)) (Variables|Default|GetTowerIndex))
    (else
      (Variables|Default|SetBuildMode false)
      (Default|UnselectSlot (Variables|/Game/Blueprints/GUI/WBP_Main.WBP_Main_C|GetWB_TrapBook (Variables|Default|GetMain%20Widget)))
      ;[1 0 0.7789] reset everything
      (CallFunction|ResetBuildMode)
      (if (Variables|Default|GetDestroyMode)
        (Variables|Default|SetDestroyMode false)
        (Utilities|IsValid (Utilities|Array|Get(acopy) (Variables|Default|GetD_Component))
          (:Is%20Valid
            (for _array_element_2 (Variables|Default|GetD_Component)
              (Rendering|Material|SetMaterial _array_element_2 0 (Variables|Default|GetD_Component_OriginalMaterial))
              (Default|Add/RemoveMappingContext (.AsBP%20Camera%20Controller (Utilities|Casting|CastToBP_CameraController (Game|GetPlayerController 0))) true "/Game/Blueprints/Controls/IMC_TrapMode.IMC_TrapMode"))))))))

(event Custom|MouseClick
  (if (Variables|Default|GetNewTrapSelected)
    (Variables|Default|SetNewTrapSelected false)
    (elif (Variables|Default|GetBuildMode)
      ;[0 0.4649 1] On click event
      (if (and (Variables|Default|GetBuildable) (> (Variables|/Game/Blueprints/GUI/WB_TrapBook.WB_TrapBook_C|GetChildrenCount (Variables|/Game/Blueprints/GUI/WBP_Main.WBP_Main_C|GetWB_TrapBook (Variables|Default|GetMain%20Widget))) 0))
        (Variables|/Game/Blueprints/LevelElements/BP_corridor.BP_corridor_C|SetHaveTrap (Variables|Default|GetTargetedCorridor) true)
        (bind _returnvalue (Game|SpawnActorfromClass (.BluePrint (Utilities|Struct|BreakST_TrapType (Utilities|Array|Get(acopy) (Variables|Default|GetDT_trap) (Variables|Default|GetTowerIndex)))) (Variables|Default|GetBuild%20Preview%20Transform) "AlwaysSpawn" "MultiplyWithRoot" 0 0))
        (bind _asbp_build_master (Utilities|Casting|CastToBP_BuildMaster _returnvalue))
        (Default|GetCoriRef _asbp_build_master (Variables|Default|GetTargetedCorridor))
        (Variables|/Game/Blueprints/Camera/BP_CameraActor.BP_CameraActor_C|SetNew_Trap (.AsBP%20Camera%20Actor (Utilities|Casting|CastToBP_CameraActor (Variables|Default|GetPlayer))) _returnvalue)
        (Default|ReduceCounter (Variables|/Game/Blueprints/GUI/WBP_Main.WBP_Main_C|GetWB_TrapBook (Variables|Default|GetMain%20Widget)))
        ;[1 0 0.7789] reset everything
        (CallFunction|ResetBuildMode)
        (if (Variables|Default|GetDestroyMode)
          (Variables|Default|SetDestroyMode false)
          (Utilities|IsValid (Utilities|Array|Get(acopy) (Variables|Default|GetD_Component))
            (:Is%20Valid
              (for _array_element (Variables|Default|GetD_Component)
                (Rendering|Material|SetMaterial _array_element 0 (Variables|Default|GetD_Component_OriginalMaterial))
                (Default|Add/RemoveMappingContext (.AsBP%20Camera%20Controller (Utilities|Casting|CastToBP_CameraController (Game|GetPlayerController 0))) true "/Game/Blueprints/Controls/IMC_TrapMode.IMC_TrapMode"))))))
      (elif (Variables|Default|GetDestroyMode)
        (Utilities|IsValid (Variables|Default|GetD_Actor)
          (:Is%20Valid
            (bind _asbp_build_master_2 (Utilities|Casting|CastToBP_BuildMaster (Variables|Default|GetD_Actor))
              (:then
                (Variables|/Game/Blueprints/LevelElements/BP_corridor.BP_corridor_C|SetHaveTrap (Variables|/Game/Blueprints/Interactibles/Tower/BP_BuildMaster.BP_BuildMaster_C|GetCorridorRef _asbp_build_master_2) false))
              (:CastFailed
                _))
            (Actor|DestroyActor (Variables|Default|GetD_Actor))))))))

(event EventBeginPlay
  ;[1 1 1] Event begin play
  (bind _asbp_game_mode (Utilities|Casting|CastToBP_GameMode (Game|GetGameMode)))
  (Variables|Default|SetGame%20Mode%20Ref _asbp_game_mode)
  (bind _asbp_camera_actor (Utilities|Casting|CastToBP_CameraActor (Components|GetOwner)))
  (Variables|Default|SetPlayer _asbp_camera_actor)
  (Variables|Default|SetCamera (Variables|/Script/Engine.CameraActor|GetCameraComponent _asbp_camera_actor))
  (bind _outrownames (DataTable|GetDataTableRowNames "/Game/Blueprints/Interactibles/Tower/DT_TrapType.DT_TrapType"))
  (for _array_element _outrownames
    (bind _returnvalue (Utilities|GetDataTableRow "/Game/Blueprints/Interactibles/Tower/DT_TrapType.DT_TrapType" _array_element)
      (:then
        (Utilities|Array|Add (Variables|Default|GetDT_trap) _returnvalue))))
  (Utilities|FlowControl|Delay 0.2)
  (Default|GetBPBueldRef (Variables|/Game/Blueprints/GUI/WBP_Main.WBP_Main_C|GetWB_TrapBook (Variables|Default|GetMain%20Widget)) self))

(event EventTick
  (params (DeltaSeconds :type Float%20%28single-precision%29))
  (bind _self self)
  (bind _main_widget (Variables|Default|GetMain%20Widget))
  (bind _wb_trapbook (Variables|/Game/Blueprints/GUI/WBP_Main.WBP_Main_C|GetWB_TrapBook _main_widget))
  ;[1 0.9077 0] Event Tick
  (if (Utilities|Enum|Equal(Enum) (Variables|/Game/Blueprints/BP_GameMode.BP_GameMode_C|GetE_GameState (Variables|Default|GetGame%20Mode%20Ref)) "NewEnumerator1")
    (if (Variables|Default|GetBuildMode)
      (CallFunction|PreviewLook)
      (else
        (CallFunction|DestroyMode)))
    (else
      (CallFunction|ResetBuildMode)
      (Components|Tick|SetComponentTickEnabled _self false)
      (Components|Activation|SetActive _self false false)
      (Widget|SetIsEnabled _wb_trapbook false)
      (Widget|SetVisibility _wb_trapbook "Hidden"))))

(fn Add/RemoveMappingContext
  (params (Remove :type Boolean) (Target%20Context :type Input%20Mapping%20Context%20Object%20Reference)))