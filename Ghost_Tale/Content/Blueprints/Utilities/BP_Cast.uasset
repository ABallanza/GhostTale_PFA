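; Component on BP_CameraActor that handles placing spells (towers) in build mode, choosing among DT_SpellType rows by mouse wheel or spell book.
; During one game state, Tick traces under the cursor, marking the spot unbuildable over an existing BP_Spell.
; A recursive trace ignores spells to position a range-scaled cylinder preview, whose material shows validity.
; Clicking spawns the selected spell if buildable; right-click exits build mode, clearing the preview.
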(event Custom|ResetBuildMode
  (bind _towerindex (Variables|Default|GetTowerIndex))
  (bind _dt_spell (Variables|Default|GetDT_Spell))
  (bind _output (Utilities|Array|Get(acopy) _dt_spell _towerindex))
  (bind _spellrange (Utilities|Struct|BreakST_SpellType _output))
  ;[0 1 0.4408] Raycast for affichage
  (Utilities|Array|Clear (Variables|Default|GetIgnoredElement))
  (bind _preview_mesh (Variables|Components|GetPreview%20Mesh)
    (:then
      (Components|StaticMesh|SetStaticMesh _preview_mesh 0)
      (Variables|Components|SetPreview%20Mesh 0)
      (Utilities|FlowControl|DoOnce false) ; enters at Reset
    )
    (:else)))

(event Custom|MWD
  ;[0 0.54 1] Mouse Wheel event
  (if (< (+ (Variables|Default|GetTowerIndex) -1) 0)
    (Variables|Default|SetTowerIndex (+ (Utilities|Array|Length (Variables|Default|GetDT_Spell)) -1))
    (else
      (Variables|Default|SetTowerIndex (+ (Variables|Default|GetTowerIndex) -1))))
  (Development|PrintString "franh")
  (Default|OnWheelEvent (Variables|/Game/Blueprints/GUI/WBP_Main.WBP_Main_C|GetWB_SpellBook (Variables|Default|GetMain%20Widget)) (Variables|Default|GetTowerIndex))
  (Variables|Default|SetBuildMode true)
  (CallFunction|ResetBuildMode))

(event Custom|MWU
  ;[0 0.54 1] Mouse Wheel event
  (if (> (+ (Variables|Default|GetTowerIndex) 1) (+ (Utilities|Array|Length (Variables|Default|GetDT_Spell)) -1))
    (Variables|Default|SetTowerIndex 0)
    (else
      (Variables|Default|SetTowerIndex (+ (Variables|Default|GetTowerIndex) 1))))
  (Development|PrintString "franh")
  (Default|OnWheelEvent (Variables|/Game/Blueprints/GUI/WBP_Main.WBP_Main_C|GetWB_SpellBook (Variables|Default|GetMain%20Widget)) (Variables|Default|GetTowerIndex))
  (Variables|Default|SetBuildMode true)
  (CallFunction|ResetBuildMode))

(event Custom|AffichageRayCast
  (params (Actor%20to%20Ignore :type Array%20of%20Actor%20Object%20References))
  (bind _returnvalue (Game|GetPlayerController 0))
  (bind _towerindex (Variables|Default|GetTowerIndex))
  (bind _dt_spell (Variables|Default|GetDT_Spell))
  (bind (_worldlocation _worlddirection) (Game|Player|ConvertMouseLocationToWorldSpace _returnvalue))
  (bind _output (Utilities|Array|Get(acopy) _dt_spell _towerindex))
  (bind _spellrange (Utilities|Struct|BreakST_SpellType _output))
  ;[0 1 0.4408] Raycast for affichage
  (bind (_outhit _returnvalue_2) (Collision|LineTraceByChannel _worldlocation (+ _worlddirection (* _worlddirection 2e+03)) "TraceTypeQuery1" false Actor%20to%20Ignore "None"))
  (if _returnvalue_2
    (bind _asbp_spell (Utilities|Casting|CastToBP_Spell (.HitActor (Collision|BreakHitResult _outhit)))
      (:then
        (Utilities|Array|Add (Variables|Default|GetIgnoredElement) _asbp_spell)
        (CallFunction|AffichageRayCast (Variables|Default|GetIgnoredElement)))
      (:CastFailed
        (Utilities|FlowControl|Sequence
          (:then_0
            (Utilities|FlowControl|DoOnce false
              (:Completed
                (bind _returnvalue_3 (Game|AddComponentbyClass (.AsActor (Utilities|Casting|CastToActor (Variables|Default|GetPlayer))) "/Script/Engine.StaticMeshComponent" false (Variables|Default|GetBuild%20Preview%20Transform)))
                (bind _output_get (Variables|Components|SetPreview%20Mesh _returnvalue_3))
                (Components|StaticMesh|SetStaticMesh _output_get "/Engine/BasicShapes/Cylinder.Cylinder")
                (Transformation|SetRelativeScale3D (Variables|Components|GetPreview%20Mesh) (Math|Vector|MakeVector _spellrange _spellrange 1.0))
                (Collision|SetCollisionEnabled (Variables|Components|GetPreview%20Mesh) "NoCollision")
                (if (Variables|Default|GetBuildable)
                  (Rendering|Material|SetMaterial (Variables|Components|GetPreview%20Mesh) 0 "/Game/Blueprints/Interactibles/Tower/Visual/MI_TowerPreview.MI_TowerPreview")
                  (else
                    (Rendering|Material|SetMaterial (Variables|Components|GetPreview%20Mesh) 0 "/Game/Blueprints/Interactibles/Tower/Visual/MI_TowerDestroy.MI_TowerDestroy"))))))
          (:then_1
            (bind _output_get_2 (Variables|Default|SetBuild%20Preview%20Transform (Math|Transform|MakeTransform (.Location (Collision|BreakHitResult _outhit)) "0, 0, 0" "1.000000,1.000000,1.000000")))
            (Transformation|SetWorldTransform (Variables|Components|GetPreview%20Mesh) _output_get_2 false false)))))))

(event Custom|ManualSwitch
  (params (index :type Integer))
  ;[0 0.54 1] Mouse Wheel event
  (Variables|Default|SetTowerIndex index)
  (Variables|Default|SetNewSpellSelected true)
  (Variables|Default|SetBuildMode true)
  (CallFunction|ResetBuildMode))

(event Custom|PreviewLook
  (bind _returnvalue (Game|GetPlayerController 0))
  (bind (_worldlocation _worlddirection) (Game|Player|ConvertMouseLocationToWorldSpace _returnvalue))
  ;[0 1 0.07869] Raycast for detection
  (bind (_outhit _returnvalue_2) (Collision|LineTraceByChannel _worldlocation (+ _worlddirection (* _worlddirection 2e+03)) "TraceTypeQuery1" false 0 "None"))
  (if _returnvalue_2
    (if (.bSuccess (Utilities|Casting|CastToBP_Spell (.HitActor (Collision|BreakHitResult _outhit))))
      (if (Variables|Default|GetBuildable)
        (CallFunction|ResetBuildMode))
      (Variables|Default|SetBuildable false)
      (else
        (if (Variables|Default|GetBuildable)
          _
          (else
            (CallFunction|ResetBuildMode)))
        (Variables|Default|SetBuildable true)))
    (Utilities|Array|Add (Variables|Default|GetIgnoredElement) (.AsBP%20Spell (Utilities|Casting|CastToBP_Spell (.HitActor (Collision|BreakHitResult _outhit)))))
    (CallFunction|AffichageRayCast (Variables|Default|GetIgnoredElement))))

(event Custom|Get%20Widget%20Ref
  (params (Widget%20Ref :type WBP%20Main%20Object%20Reference))
  (Variables|Default|SetMain%20Widget Widget%20Ref))

(event Custom|MouseR%20click
  ;[0 0.03631 1] Enable-Disable buildmode
  (Variables|Default|SetBuildMode false)
  (Default|UnselectSlot (Variables|/Game/Blueprints/GUI/WBP_Main.WBP_Main_C|GetWB_SpellBook (Variables|Default|GetMain%20Widget)))
  ;[1 0 0.7789] reset everything
  (CallFunction|ResetBuildMode)
  (if (Variables|Default|GetDestroyMode)
    (Variables|Default|SetDestroyMode false)
    (Utilities|IsValid (Utilities|Array|Get(acopy) (Variables|Default|GetD_Component))
      (:Is%20Valid
        (for _array_element (Variables|Default|GetD_Component)
          (Rendering|Material|SetMaterial _array_element 0 (Variables|Default|GetD_Component_OriginalMaterial)))))))

(event Custom|Build
  ;[0 0.03631 1] Enable-Disable buildmode
  (if (not (Variables|Default|GetBuildMode))
    (Variables|Default|SetBuildMode true)
    (else
      (Variables|Default|SetBuildMode false)
      (Default|UnselectSlot (Variables|/Game/Blueprints/GUI/WBP_Main.WBP_Main_C|GetWB_SpellBook (Variables|Default|GetMain%20Widget)))
      ;[1 0 0.7789] reset everything
      (CallFunction|ResetBuildMode)
      (if (Variables|Default|GetDestroyMode)
        (Variables|Default|SetDestroyMode false)
        (Utilities|IsValid (Utilities|Array|Get(acopy) (Variables|Default|GetD_Component))
          (:Is%20Valid
            (for _array_element (Variables|Default|GetD_Component)
              (Rendering|Material|SetMaterial _array_element 0 (Variables|Default|GetD_Component_OriginalMaterial)))))))))

(event Custom|MouseClick
  ;[0 0.4649 1] On click event
  (if (Variables|Default|GetNewSpellSelected)
    (Variables|Default|SetNewSpellSelected false)
    (elif (Variables|Default|GetBuildMode)
      (if (Variables|Default|GetBuildable)
        (Game|SpawnActorfromClass (.BP_Spell (Utilities|Struct|BreakST_SpellType (Utilities|Array|Get(acopy) (Variables|Default|GetDT_Spell) (Variables|Default|GetTowerIndex)))) (Variables|Default|GetBuild%20Preview%20Transform) "AlwaysSpawn" "MultiplyWithRoot" 0 0)
        ;[1 0 0.7789] reset everything
        (CallFunction|ResetBuildMode)
        (if (Variables|Default|GetDestroyMode)
          (Variables|Default|SetDestroyMode false)
          (Utilities|IsValid (Utilities|Array|Get(acopy) (Variables|Default|GetD_Component))
            (:Is%20Valid
              (for _array_element (Variables|Default|GetD_Component)
                (Rendering|Material|SetMaterial _array_element 0 (Variables|Default|GetD_Component_OriginalMaterial))))))))))

(event EventBeginPlay
  ;[1 1 1] Event begin play
  (bind _asbp_game_mode (Utilities|Casting|CastToBP_GameMode (Game|GetGameMode)))
  (Variables|Default|SetGame%20Mode%20Ref _asbp_game_mode)
  (bind _asbp_camera_actor (Utilities|Casting|CastToBP_CameraActor (Components|GetOwner)))
  (Variables|Default|SetPlayer _asbp_camera_actor)
  (Variables|Default|SetCamera (Variables|/Script/Engine.CameraActor|GetCameraComponent _asbp_camera_actor))
  (bind _outrownames (DataTable|GetDataTableRowNames "/Game/Blueprints/Interactibles/Spell/DT_SpellType.DT_SpellType"))
  (for _array_element _outrownames
    (bind _returnvalue (Utilities|GetDataTableRow "/Game/Blueprints/Interactibles/Spell/DT_SpellType.DT_SpellType" _array_element)
      (:then
        (Utilities|Array|Add (Variables|Default|GetDT_Spell) _returnvalue))))
  (Utilities|FlowControl|Delay 0.2)
  (bind _asbp_camera_controller (Utilities|Casting|CastToBP_CameraController (Game|GetPlayerController 0))))

(event EventTick
  (params (DeltaSeconds :type Float%20%28single-precision%29))
  ;[1 0.9077 0] Event Tick
  (if (Utilities|Enum|Equal(Enum) (Variables|/Game/Blueprints/BP_GameMode.BP_GameMode_C|GetE_GameState (Variables|Default|GetGame%20Mode%20Ref)) "NewEnumerator2")
    (if (Variables|Default|GetBuildMode)
      (CallFunction|PreviewLook))))