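; BP_Clean is a component on BP_CameraActor that detects which BP_Room is under the mouse cursor, apparently for a cleaning interaction.
; BeginPlay disables its tick and caches game mode, owner and camera; when ticking, PreviewLook traces from the cursor and stores or clears the hovered room.
; MouseClick and AddRemoveMappingContext are empty stubs, and disconnected logic would spawn a widget at the room and remove IMC_TrapMode.
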(event Custom|PreviewLook
  (bind _returnvalue (Game|GetPlayerController 0))
  (bind (_worldlocation _worlddirection) (Game|Player|ConvertMouseLocationToWorldSpace _returnvalue))
  ;[0 1 0.07869] Raycast for detection
  (bind (_outhit _returnvalue_2) (Collision|LineTraceByChannel _worldlocation (+ _worldlocation (* _worlddirection 5e+03)) "TraceTypeQuery1" false 0 "None" true "(R=0.848955,G=0.000000,B=1.000000,A=1.000000)"))
  (if _returnvalue_2
    (bind _asbp_room (Utilities|Casting|CastToBP_Room (.HitActor (Collision|BreakHitResult _outhit)))
      (:then
        (Variables|Default|SetAs%20BP%20Room _asbp_room))
      (:CastFailed
        (Variables|Default|SetAs%20BP%20Room 0 :!label _label)))
    (else
      (goto _label))))

(event Custom|Get%20Widget%20Ref
  (params (Widget%20Ref :type WBP%20Main%20Object%20Reference))
  (Variables|Default|SetMain%20Widget Widget%20Ref))

(event Custom|MouseClick
  ;[0 0.4649 1] On click event
)

(event EventBeginPlay
  ;[1 1 1] Event begin play
  (Components|Tick|SetComponentTickEnabled false)
  (bind _asbp_game_mode (Utilities|Casting|CastToBP_GameMode (Game|GetGameMode)))
  (Variables|Default|SetGame%20Mode%20Ref _asbp_game_mode)
  (bind _asbp_camera_actor (Utilities|Casting|CastToBP_CameraActor (Components|GetOwner)))
  (Variables|Default|SetPlayer _asbp_camera_actor)
  (Variables|Default|SetCamera (Variables|/Script/Engine.CameraActor|GetCameraComponent _asbp_camera_actor)))

(event EventTick
  (params (DeltaSeconds :type Float%20%28single-precision%29))
  ;[1 0.9077 0] Event Tick
  (CallFunction|PreviewLook))

(fn Add/RemoveMappingContext
  (params (Remove :type Boolean) (Target%20Context :type Input%20Mapping%20Context%20Object%20Reference)))