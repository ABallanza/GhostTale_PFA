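; Spell actor with a limited lifetime, apparently a base for specific spells.
; SetupStat waits for the given lifetime, calls the empty BeforeDestroy hook, then destroys the actor.
; A local Timeline macro, unused in the event graph, imitates a timeline with play, stop and reverse inputs.
; Its gate loop steps position by world delta seconds up to a length, with no delay node between steps.
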(event Custom|Setup%20Stat
  (params (lifetime :type Integer))
  (Utilities|FlowControl|Delay (Math|Conversions|ToFloat(Integer) lifetime))
  (CallFunction|BeforeDestroy)
  (Actor|DestroyActor))

(event Custom|BeforeDestroy)

(event EventBeginPlay)

(event Collision|EventActorBeginOverlap
  (params (OtherActor :type Actor%20Object%20Reference)))

(event EventTick
  (params (DeltaSeconds :type Float%20%28single-precision%29)))

(fn ConstructionScript)