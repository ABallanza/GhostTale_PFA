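; BP_Spiderpell is a spell area actor that slows adventurers inside its sphere.
; On overlap, it divides each BP_AdventurerClass walk speed by SpeedDivisor and tracks the character in an array.
; Leaving the sphere multiplies the speed back and removes the character from that array.
; The BeforeDestroy event restores speed for everyone still tracked and clears the array.
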(event OnComponentBeginOverlap(Sphere)
  (params (OverlappedComponent :type Primitive%20Component%20Object%20Reference) (OtherActor :type Actor%20Object%20Reference) (OtherComp :type Primitive%20Component%20Object%20Reference) (OtherBodyIndex :type Integer) (bFromSweep :type Boolean) (SweepResult :type Hit%20Result%20Structure%20%28by%20ref%29))
  (bind _asbp_adventurer_class (Utilities|Casting|CastToBP_AdventurerClass OtherActor))
  (Variables|/Script/Engine.CharacterMovementComponent|SetMaxWalkSpeed (Variables|/Script/Engine.Character|GetCharacterMovement _asbp_adventurer_class) (/ (Variables|/Script/Engine.CharacterMovementComponent|GetMaxWalkSpeed (Variables|/Script/Engine.Character|GetCharacterMovement _asbp_adventurer_class)) (Variables|Default|GetSpeedDivisor)))
  (Utilities|Array|Add (Variables|Default|GetAs%20BP%20Adventurer%20Class) _asbp_adventurer_class))

(event OnComponentEndOverlap(Sphere)
  (params (OverlappedComponent :type Primitive%20Component%20Object%20Reference) (OtherActor :type Actor%20Object%20Reference) (OtherComp :type Primitive%20Component%20Object%20Reference) (OtherBodyIndex :type Integer))
  (bind _asbp_adventurer_class (Utilities|Casting|CastToBP_AdventurerClass OtherActor))
  (Variables|/Script/Engine.CharacterMovementComponent|SetMaxWalkSpeed (Variables|/Script/Engine.Character|GetCharacterMovement _asbp_adventurer_class) (* (Variables|/Script/Engine.CharacterMovementComponent|GetMaxWalkSpeed (Variables|/Script/Engine.Character|GetCharacterMovement _asbp_adventurer_class)) (Variables|Default|GetSpeedDivisor)))
  (Utilities|Array|RemoveItem (Variables|Default|GetAs%20BP%20Adventurer%20Class) _asbp_adventurer_class))

(event EventBeginPlay
  (|CallParentFunction) ; This node is disabled and will not be called.\nDrag off pins to build functionality.
)

(event Collision|EventActorBeginOverlap
  (params (OtherActor :type Actor%20Object%20Reference))
  (|CallParentFunction OtherActor) ; This node is disabled and will not be called.\nDrag off pins to build functionality.
)

(event EventTick
  (params (DeltaSeconds :type Float%20%28single-precision%29))
  (|CallParentFunction DeltaSeconds) ; This node is disabled and will not be called.\nDrag off pins to build functionality.
)

(event EventBeforeDestroy
  (for _array_element (Variables|Default|GetAs%20BP%20Adventurer%20Class)
    (Variables|/Script/Engine.CharacterMovementComponent|SetMaxWalkSpeed (Variables|/Script/Engine.Character|GetCharacterMovement _array_element) (* (Variables|/Script/Engine.CharacterMovementComponent|GetMaxWalkSpeed (Variables|/Script/Engine.Character|GetCharacterMovement _array_element)) (Variables|Default|GetSpeedDivisor))))
  (Utilities|Array|Clear (Variables|Default|GetAs%20BP%20Adventurer%20Class)))

(fn ConstructionScript
  (|CallParentFunction))