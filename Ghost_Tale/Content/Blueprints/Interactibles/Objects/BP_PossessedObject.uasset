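; Interactable prop that the player can possess with an effect to scare the wizard, warrior or thief who uses it.
; Its data table row supplies meshes, sounds, effect options and weights for picking an adventurer.
; Clicking opens a radial effect menu, flashes red if already possessed, or resets and cleans a dirty object.
; Adventurer use triggers the effect or normal animation, dirties it and plays chained sounds; timeline scaling handles mesh morphs.
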(event OnClicked(StaticBody)
  (params (TouchedComponent :type Primitive%20Component%20Object%20Reference) (ButtonPressed :type Key%20Structure :default "None"))
  ;[1 0.9127 0.4111 0.4] Interaction
  ;;[1 0.6797 0.1562] Avec le joueur
  ;;;[1 0.6429 0] Quand on clique sur l'acteur
  (if (Variables|State|GetIsDirty)
    (CallFunction|ResetDefaultState)
    (elif (Variables|State|GetIs%20Possessed)
      (CallFunction|WrongClick)
      (else
        (CallFunction|PlayerInteract)))))

(event Custom|Player%20Interact
  ;[1 0.9127 0.4111 0.4] Interaction
  ;;[1 0.6797 0.1562] Avec le joueur
  ;;;[0.5417 0.2808 0] Ouvre le Menu Radial
  (bind _returnvalue (UserInterface|CreateWidget "/Game/Blueprints/GUI/WBP_PossessedObject.WBP_PossessedObject_C" 0 (.EffectData (Utilities|Struct|BreakST_PossessedObjects (Variables|ObjectData|GetData%20Table%20Row))) 1.5e+02 self))
  (UserInterface|Viewport|AddtoViewport _returnvalue 0)
  (Default|SetPosition _returnvalue (Transformation|GetActorLocation)))

(event Custom|Adventurer%20Interact
  (params (Adventurer :type BP%20Adventurer%20Class%20Object%20Reference))
  (bind _selected_effect (Variables|ObjectData|GetSelected%20Effect))
  (if (Variables|State|GetIs%20Possessed)
    ;[1 0.9127 0.4111 0.4] Interaction
    ;;[0.952 1 0.005372] Avec les aventuriers - Has been used sert aussi à savoir si l'objet est sale ou pas pour le moment
    (bind _output_get (Variables|Références|SetAdventurerInterract Adventurer))
    (Default|ActivateEffect _selected_effect _output_get (CallFunction|GetFearAmount _selected_effect))
    (else
      (CallFunction|NonePossessedUse)
      (CallFunction|SetHasBeenUsed true)))
  (if (Variables|State|GetIsDirty)
    _
    (else
      (Default|MakeDirt (Variables|Références|GetGame%20Mode%20Ref) 1.0)
      (Variables|State|SetIsDirty true)))
  ;;[1 0.3587 0] Joue les sons de l'objet (en fonction de s'il est maudit ou pas)
  (Utilities|FlowControl|Delay (Default|GetDelayBeforePlaySound (Variables|ObjectData|GetSelected%20Effect)))
  (CallFunction|PlaySound (Utilities|Array|Get(acopy) (Variables|Default|GetAll%20Sounds) (Variables|Default|GetIndex%20Sound%20To%20Play)) (Transformation|GetActorLocation)))

(event Custom|Reset%20Mesh
  (bind _static_body (Variables|Default|GetStatic%20Body))
  (bind _data_table_row (Variables|ObjectData|GetData%20Table%20Row))
  (bind (_name _effectdata _manacost _fearamount _staticbody _skeletalbody _material) (Utilities|Struct|BreakST_PossessedObjects _data_table_row))
  ;[1 1 1] Nettoie l'Objet (en cours de dev)
  (Variables|Utilitaires|SetCleaning true)
  (CallFunction|MorphMeshin)
  (Components|StaticMesh|SetStaticMesh _static_body _staticbody)
  (Rendering|Material|SetMaterial _static_body 0 _material)
  (Rendering|Material|SetOverlayMaterial _static_body "/Game/GA/VFX/Materials/M_Outline.M_Outline" :!class /Script/Engine.MeshComponent)
  (Utilities|FlowControl|Delay 0.1)
  (bind _returnvalue (Niagara|SpawnSystemAttached "/Game/GA/VFX/NiagaraSystem/NS_Item_Maudissable.NS_Item_Maudissable" _static_body "None" (Transformation|GetWorldLocation _static_body) (Transformation|GetWorldRotation _static_body) "KeepWorldPosition" false))
  (Utilities|FlowControl|Delay 0.2)
  (Components|DestroyComponent _returnvalue)
  (CallFunction|MorphMeshOut)
  (Utilities|FlowControl|Delay 5.0)
  (Variables|Utilitaires|SetCleaning false))

(event Custom|Morph%20Mesh%20Out
  (bind _selected_effect (Variables|ObjectData|GetSelected%20Effect))
  (bind (_delay_before_animation _animation _loop_animation) (Default|GetAnimationData _selected_effect))
  ;[0.01246 0.4479 0.2022 0.5] Morphing (juste une timeligne pour rescale le mesh, impossible à faire dans le PDA_Effect)
  (Variables|Utilitaires|SetMorph%20Target (CallFunction|SetMorphTarget true))
  (bind _alpha (Timeline|Scale%20Mesh ReverseFromEnd)
    (:Update
      (Transformation|SetWorldScale3D (Variables|Utilitaires|GetMorph%20Target) (Math|Vector|MakeVector _alpha _alpha _alpha)))
    (:Finished
      ;;[0 1 0.635 0.7] Evite de recommencer le cycle éternellement
      (if (not (Variables|Utilitaires|GetCleaning))
        (if (Variables|State|GetIs%20Morph)
          ;;[0.776 0.7166 0.0002] Destroy le "pouf" VFX
          (Default|DestroyVFX _selected_effect)
          ;;[1 0.4531 0 0.8] Joue l'Animation
          (Utilities|FlowControl|Delay _delay_before_animation)
          (Default|PlayAnimation _selected_effect (Variables|Default|GetSkeletal%20Body) _animation _loop_animation)
          (else
            (Variables|State|SetIs%20Morph true)
            (CallFunction|MorphMeshOut)
            ;;[0 0.3208 1 0.2] Appelle le VFX "pouf"
            (Utilities|FlowControl|Delay 0.2)
            (Default|MorphObject (Variables|ObjectData|GetSelected%20Effect))))))))

(event Custom|Cleaning%20object
  ;[1 1 1] Nettoie l'Objet (en cours de dev)
  (if (Variables|State|GetIsDirty)
    (Default|TidyUp (Variables|Références|GetGame%20Mode%20Ref) 1.0)
    (Variables|State|SetIsDirty false)
    (CallFunction|CleanObject)))

(event Custom|NonePossessedUse
  (bind _data_table_row (Variables|ObjectData|GetData%20Table%20Row))
  (bind _skeletal_body (Variables|Default|GetSkeletal%20Body))
  (bind (_name _effectdata _manacost _fearamount _staticbody _skeletalbody _material _animation _loopanimation) (Utilities|Struct|BreakST_PossessedObjects _data_table_row))
  ;[1 0.9127 0.4111 0.4] Interaction
  ;;[0.952 1 0.005372] Avec les aventuriers - Has been used sert aussi à savoir si l'objet est sale ou pas pour le moment
  ;;;[0.5149 1 0] Utilisation par un aventurier si l'objet n'est pas possédé
  (Transformation|SetWorldScale3D (Variables|Default|GetStatic%20Body) "0.010000,0.010000,0.010000")
  (Transformation|SetWorldScale3D _skeletal_body "1.000000,1.000000,1.000000")
  (Components|Animation|PlayAnimation _skeletal_body _animation _loopanimation))

(event Custom|PlaySound
  (params (Sound :type Sound%20Base%20Object%20Reference) (Location :type Vector))
  (bind _new_index (CallFunction|SetSoundtoPlay))
  (bind _data_table_row (Variables|ObjectData|GetData%20Table%20Row))
  (bind _selected_effect (Variables|ObjectData|GetSelected%20Effect))
  (bind _sound (Utilities|Struct|BreakST_PossessedObjects _data_table_row))
  (bind _sounds (Default|GetSoundMap _selected_effect))
  (bind _returnvalue (== _new_index 0))
  (bind (_value _returnvalue_2) (Utilities|Map|Find _sound Sound))
  (bind _returnvalue_3 (not _returnvalue))
  (bind (_value_2 _returnvalue_4) (Utilities|Map|Find _sounds Sound))
  ;[0.2877 0.4375 0 0.5] Sons de l'objet
  ;;[1 0.6402 0] Joue le son à l'endroit choisi
  (Audio|PlaySoundatLocation Sound Location "0, 0, 0" 1.0 1.0 0.0 0 0 0 0)
  ;;[0 1 0.1856] Vérifie si le son actuel a un délai avant de lancer le son suivant (Version Possédée)
  (if (Variables|State|GetIs%20Possessed)
    (if (and _returnvalue_4 _returnvalue_3)
      ;;[1 0.7605 0.3333] Met un délai avant de jouer le son suivant
      (Utilities|FlowControl|Delay _value_2)
      (CallFunction|PlaySound (Utilities|Array|Get(acopy) (Variables|Default|GetAll%20Sounds) (Variables|Default|GetIndex%20Sound%20To%20Play)) (Transformation|GetActorLocation) :!label _label))
    (else
      ;;[0.6646 1 0] Vérifie si le son actuel a un délai avant de lancer le son suivant (Version Normale)
      (if (and _returnvalue_3 _returnvalue_2)
        (Utilities|FlowControl|Delay _value)
        (goto _label)))))

(event Custom|Select%20New%20Adventurer
  ;[0.5471 0.1042 1] Choisit un aventurier qui doit intéragir avec l'objet
  (bind _selected_adventurer (CallFunction|SelectAdventurer))
  (Variables|Références|SetAdventurerInterract _selected_adventurer))

(event Custom|WrongClick
  (bind _static_body (Variables|Default|GetStatic%20Body))
  ;[1 0.9127 0.4111 0.4] Interaction
  ;;[1 0.6797 0.1562] Avec le joueur
  ;;;[1 0.05682 0] Clignote en Rouge
  (bind _alpha (Timeline|Material%20Blick PlayFromStart)
    (:Update
      (if (>= _alpha 1.0)
        (Rendering|Material|SetOverlayMaterial _static_body "/Game/GA/VFX/Materials/MI_Outline_Red.MI_Outline_Red" :!class /Script/Engine.MeshComponent)
        (else
          (Rendering|Material|SetOverlayMaterial _static_body "/Game/GA/VFX/Materials/MI_Outline_Purple.MI_Outline_Purple" :!class /Script/Engine.MeshComponent))))
    (:Finished
      (Rendering|Material|SetOverlayMaterial (Variables|Default|GetStatic%20Body) "/Game/GA/VFX/Materials/MI_Outline_Purple.MI_Outline_Purple" :!class /Script/Engine.MeshComponent))))

(event Custom|SetupAdvList
  (bind _game_mode_ref (Variables|Références|GetGame%20Mode%20Ref))
  ;[1 1 1 0.2] Event Begin Play
  ;;[0.2604 0.2604 0.2604 0.8] Obtient la référence de tous les aventuriers et les place dans un tableau
  (Variables|Références|SetWizard%20Ref (Default|GetWizard _game_mode_ref))
  (Variables|Références|SetWarrior%20Ref (Default|GetWarrior _game_mode_ref))
  (Variables|Références|SetThief%20Ref (Default|GetThief _game_mode_ref))
  (Variables|Références|SetAllAdventurer (Utilities|Array|MakeArray (Variables|Références|GetWizard%20Ref) (Variables|Références|GetWarrior%20Ref) (Variables|Références|GetThief%20Ref))))

(event Custom|Become%20Possessed
  (params (Selected%20Effect :type PDA%20Effects%20Object%20Reference))
  ;[1 0 0.6195] Become Possessed
  (bind _output_get (Variables|ObjectData|SetSelected%20Effect Selected%20Effect))
  (Default|SetOwner _output_get self)
  (Variables|State|SetIs%20Possessed true)
  (Rendering|Material|SetOverlayMaterial (Variables|Default|GetStatic%20Body) "/Game/GA/VFX/Materials/MI_Outline_Purple.MI_Outline_Purple" :!class /Script/Engine.MeshComponent)
  (bind _keys (Utilities|Map|Keys (Default|GetSoundMap (Variables|ObjectData|GetSelected%20Effect))))
  (Variables|Default|SetAll%20Sounds _keys))

(event Custom|Morph%20Mesh%20In
  (bind _selected_effect (Variables|ObjectData|GetSelected%20Effect))
  (bind (_delay_before_animation _animation _loop_animation) (Default|GetAnimationData _selected_effect))
  ;[0.01246 0.4479 0.2022 0.5] Morphing (juste une timeligne pour rescale le mesh, impossible à faire dans le PDA_Effect)
  (Variables|Utilitaires|SetMorph%20Target (CallFunction|SetMorphTarget false))
  (bind _alpha (Timeline|Scale%20Mesh PlayFromStart)
    (:Update
      (Transformation|SetWorldScale3D (Variables|Utilitaires|GetMorph%20Target) (Math|Vector|MakeVector _alpha _alpha _alpha)))
    (:Finished
      ;;[0 1 0.635 0.7] Evite de recommencer le cycle éternellement
      (if (not (Variables|Utilitaires|GetCleaning))
        (if (Variables|State|GetIs%20Morph)
          ;;[0.776 0.7166 0.0002] Destroy le "pouf" VFX
          (Default|DestroyVFX _selected_effect)
          ;;[1 0.4531 0 0.8] Joue l'Animation
          (Utilities|FlowControl|Delay _delay_before_animation)
          (Default|PlayAnimation _selected_effect (Variables|Default|GetSkeletal%20Body) _animation _loop_animation)
          (else
            (Variables|State|SetIs%20Morph true)
            (CallFunction|MorphMeshOut)
            ;;[0 0.3208 1 0.2] Appelle le VFX "pouf"
            (Utilities|FlowControl|Delay 0.2)
            (Default|MorphObject (Variables|ObjectData|GetSelected%20Effect))))))))

(event Custom|Clean%20Object
  ;[1 1 1] Nettoie l'Objet (en cours de dev)
  (bind _returnvalue (Niagara|SpawnSystematLocation "/Game/GA/VFX/NiagaraSystem/NS_Clean.NS_Clean" (Transformation|GetActorLocation)))
  (Utilities|FlowControl|Delay (Variables|CleanSystem|GetClean%20VFX%20Duration))
  (Components|DestroyComponent _returnvalue))

(event Custom|Reset%20Default%20State
  ;[1 1 1] Nettoie l'Objet (en cours de dev)
  (CallFunction|ResetMesh)
  (Variables|State|SetIs%20Possessed false)
  (Variables|State|SetHas%20Been%20Used false)
  (Variables|State|SetIs%20Morph false)
  (CallFunction|CleaningObject))

(event EventBeginPlay
  ;[1 1 1 0.2] Event Begin Play
  (Utilities|FlowControl|Delay 0.2)
  (bind _asbp_game_mode (Utilities|Casting|CastToBP_GameMode (Game|GetGameMode))
    (:then
      (Variables|Références|SetGame%20Mode%20Ref _asbp_game_mode)
      (CallFunction|SetupAdvList))
    (:CastFailed
      (Development|PrintText "ERREUR GAME MODE" true true "(R=0.369792,G=0.000000,B=0.031119,A=1.000000)")))
  ;;[0.5781 0.5781 0.5781 0.8] Met à jour ses données d'objet possédé
  (bind _returnvalue (Utilities|GetDataTableRow "/Game/Blueprints/Interactibles/DT_PossessedObjects.DT_PossessedObjects" (Variables|ObjectData|GetName))
    (:then
      (bind _output_get (Variables|ObjectData|SetData%20Table%20Row _returnvalue))
      (bind _keys (Utilities|Map|Keys (.Sound (Utilities|Struct|BreakST_PossessedObjects _output_get))))
      (Variables|Default|SetAll%20Sounds _keys)
      (Utilities|FlowControl|Delay 0.2)
      (CallFunction|SelectNewAdventurer))
    (:RowNotFound
      (Development|PrintString "Row not found"))))

(fn ConstructionScript
  (bind _skeletal_body (Variables|Default|GetSkeletal%20Body))
  (bind _static_body (Variables|Default|GetStatic%20Body))
  (bind _returnvalue (Utilities|GetDataTableRow "/Game/Blueprints/Interactibles/DT_PossessedObjects.DT_PossessedObjects" (Variables|ObjectData|GetName))
    (:then
      (Components|StaticMesh|SetStaticMesh _static_body (.StaticBody (Utilities|Struct|BreakST_PossessedObjects _returnvalue)))
      (Rendering|Material|SetMaterial _static_body 0 (.Material (Utilities|Struct|BreakST_PossessedObjects _returnvalue)))
      (Rendering|Material|SetOverlayMaterial (Variables|Default|GetStatic%20Body) "/Game/GA/VFX/Materials/M_Outline.M_Outline" :!class /Script/Engine.MeshComponent)
      (if (Utilities|IsValid (.SkeletalBody (Utilities|Struct|BreakST_PossessedObjects _returnvalue)))
        (Components|SkeletalMesh|SetSkeletalMeshAsset _skeletal_body (.SkeletalBody (Utilities|Struct|BreakST_PossessedObjects _returnvalue))))
      (Transformation|SetWorldScale3D _skeletal_body "0.010000,0.010000,0.010000")
      (Rendering|Material|SetOverlayMaterial _skeletal_body "/Game/GA/VFX/Materials/M_Outline.M_Outline" :!class /Script/Engine.MeshComponent))))

(fn SetObjectEffect
  (params (Effect%20Data :type PDA%20Effects%20Object%20Reference))
  (return (Default|GetFearType Effect%20Data) (Default|GetFearVFX Effect%20Data)))

(fn SelectAdventurer
  (bind _data_table_row (Variables|ObjectData|GetData%20Table%20Row))
  (bind (_name _effectdata _manacost _fearamount _staticbody _skeletalbody _material _animation _loopanimation _tendencywizard _tendencywarrior _tendancythief) (Utilities|Struct|BreakST_PossessedObjects _data_table_row))
  (bind _array (Utilities|Array|MakeArray _tendencywizard _tendencywarrior _tendancythief))
  (bind _array_element (Utilities|Array|ForEachLoopwithBreak _array :!label _label)
    (:LoopBody
      (bind _output_get (LocalVariables|SetHas%20Chosen (Math|Random|RandomBoolwithWeight (/ _array_element 1e+02))))
      (if _output_get
        (goto _label Break)
        (else
          (Math|Integer|IncrementInt (LocalVariables|GetAdventurer%20Index)))))
    (:Completed
      (if (LocalVariables|GetHas%20Chosen)
        _
        (else
          (for (_array_element_2 _array_index) _array
            (if (> _array_element_2 (LocalVariables|GetHigher%20Value))
              (LocalVariables|SetHigher%20Value _array_element_2)
              (LocalVariables|SetAdventurer%20Index _array_index)))))
      (switch int (LocalVariables|GetAdventurer%20Index)
        (:Default
          (Development|PrintString "Hello"))
        (:0
          (return (Variables|Références|GetWizard%20Ref)))
        (:1
          (return (Variables|Références|GetWarrior%20Ref)))
        (:2
          (return (Variables|Références|GetThief%20Ref)))))))

(fn SetRoom
  (params (Room :type BP%20Room%20Object%20Reference))
  (Variables|Références|SetLinked%20Room Room))

(fn GetHasBeenUsed
  (return (Variables|State|GetHas%20Been%20Used)))

(fn GetBody
  (return (Variables|Default|GetStatic%20Body) (Variables|Default|GetSkeletal%20Body)))

(fn SetHasBeenUsed
  (params (Used? :type Boolean))
  (Variables|State|SetHas%20Been%20Used Used?)
  (Development|PrintString (Utilities|String|Append (Utilities|GetDisplayName self) " HAS BEEN USED") true true "(R=0.120157,G=1.000000,B=0.000000,A=1.000000)" 2e+01))

(fn IsMorph?
  (return (Variables|State|GetIs%20Morph)))

(fn SetMorphTarget
  (params (Out? :type Boolean))
  (if Out?
    (Utilities|IsValid (Default|GetNewSkeletal (Variables|ObjectData|GetSelected%20Effect))
      (:Is%20Valid
        (return (Variables|Default|GetSkeletal%20Body)))
      (:Is%20Not%20Valid
        _)))
  (return (Variables|Default|GetStatic%20Body)))

(fn GetFearAmount
  (params (Selected%20Effect :type PDA%20Effects%20Object%20Reference))
  (bind _data_table_row (Variables|ObjectData|GetData%20Table%20Row))
  (bind _fearamount (Utilities|Struct|BreakST_PossessedObjects _data_table_row))
  (bind (_value _returnvalue) (Utilities|Map|Find _fearamount Selected%20Effect))
  (if _returnvalue
    (return _value)
    (else
      (return 0.0))))

(fn GetManaAmount
  (params (Effect :type PDA%20Effects%20Object%20Reference))
  (bind _data_table_row (Variables|ObjectData|GetData%20Table%20Row))
  (bind _manacost (Utilities|Struct|BreakST_PossessedObjects _data_table_row))
  (bind (_value _returnvalue) (Utilities|Map|Find _manacost Effect))
  (if _returnvalue
    (return _value)
    (else
      (return 0.0))))

(fn SetSoundtoPlay
  (if (== (Variables|Default|GetIndex%20Sound%20To%20Play) (Utilities|Array|Length (Variables|Default|GetAll%20Sounds)))
    (bind _output_get (Variables|Default|SetIndex%20Sound%20To%20Play 0))
    (return _output_get)
    (else
      (bind _result (Math|Integer|IncrementInt (Variables|Default|GetIndex%20Sound%20To%20Play))
        (:%20%20
          (return _result))))))