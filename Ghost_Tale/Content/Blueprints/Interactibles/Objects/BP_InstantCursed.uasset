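; Clickable one-shot cursed object that spends mana to frighten nearby adventurers.
; A DT_InstantPossessed row selected by Name sets mesh and material at construction and supplies the mana cost.
; A sphere overlap tracks adventurers in range, who receive the object's fear type and amount on a successful click through BP_GameMode's mana check.
; Clicks without enough mana or after use blink the blue overlay outline red via a timeline.
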(event OnComponentBeginOverlap(Sphere)
  (params (OverlappedComponent :type Primitive%20Component%20Object%20Reference) (OtherActor :type Actor%20Object%20Reference) (OtherComp :type Primitive%20Component%20Object%20Reference) (OtherBodyIndex :type Integer) (bFromSweep :type Boolean) (SweepResult :type Hit%20Result%20Structure%20%28by%20ref%29))
  ;[0.4323 0.6299 1] Référence tous les personnages dans son champs d'action
  (bind _asbp_adventurer_class (Utilities|Casting|CastToBP_AdventurerClass OtherActor))
  (Utilities|Array|Add (Variables|Default|GetAdventurerInRange) _asbp_adventurer_class))

(event OnComponentEndOverlap(Sphere)
  (params (OverlappedComponent :type Primitive%20Component%20Object%20Reference) (OtherActor :type Actor%20Object%20Reference) (OtherComp :type Primitive%20Component%20Object%20Reference) (OtherBodyIndex :type Integer))
  ;[0.4323 0.6299 1] Référence tous les personnages dans son champs d'action
  (bind _asbp_adventurer_class (Utilities|Casting|CastToBP_AdventurerClass OtherActor))
  (Utilities|Array|RemoveItem (Variables|Default|GetAdventurerInRange) _asbp_adventurer_class))

(event OnClicked(Body)
  (params (TouchedComponent :type Primitive%20Component%20Object%20Reference) (ButtonPressed :type Key%20Structure :default "None"))
  (bind _data_row (Variables|Default|GetData%20Row))
  (bind _manacost (Utilities|Struct|BreakST_InstantPossessed _data_row))
  ;[0.3906 0.01751 0.1119] Déclanche son effet lorsqu'on clique dessus
  (bind _can_use (Default|TrytoUseMana (Variables|Default|GetGame%20Mode%20Ref) _manacost))
  (if (and _can_use (not (Variables|Default|GetIsUsed)))
    (Default|UseMana (Variables|Default|GetGame%20Mode%20Ref) _manacost)
    (for _array_element (Variables|Default|GetAdventurerInRange)
      (Default|Effrayed _array_element (Variables|Default|GetFear%20Type) (Variables|Default|GetFear%20Amount)))
    (Variables|Default|SetIsUsed true)
    (Development|PrintText "L'objet Fonctionne" true true "(R=0.061959,G=1.000000,B=0.023872,A=1.000000)")
    (else
      (CallFunction|RedBlink))))

(event Custom|RedBlink
  (bind _body (Variables|Default|GetBody))
  ;[1 0 0.02767] Clignote en rouge
  (bind _alpha (Timeline|Blink PlayFromStart)
    (:Update
      (if (>= _alpha 1.0)
        (Rendering|Material|SetOverlayMaterial _body "/Game/GA/VFX/Materials/MI_Outline_Red.MI_Outline_Red" :!class /Script/Engine.MeshComponent)
        (else
          (Rendering|Material|SetOverlayMaterial _body "/Game/GA/VFX/Materials/MI_Outline_Blue.MI_Outline_Blue" :!class /Script/Engine.MeshComponent))))
    (:Finished
      (Rendering|Material|SetOverlayMaterial (Variables|Default|GetBody) "/Game/GA/VFX/Materials/MI_Outline_Blue.MI_Outline_Blue" :!class /Script/Engine.MeshComponent))))

(event EventBeginPlay
  ;[1 1 1] Event Begin Play
  (bind _asbp_game_mode (Utilities|Casting|CastToBP_GameMode (Game|GetGameMode)))
  (Variables|Default|SetGame%20Mode%20Ref _asbp_game_mode)
  (bind _returnvalue (Utilities|GetDataTableRow "/Game/Blueprints/Interactibles/DT_InstantPossessed.DT_InstantPossessed" (Variables|Default|GetName))
    (:then
      (Variables|Default|SetData%20Row _returnvalue))))

(fn ConstructionScript
  (bind _body (Variables|Default|GetBody))
  ;[1 1 1] Met à jour le mesh en fonction du name (ref à la data table)
  (bind _returnvalue (Utilities|GetDataTableRow "/Game/Blueprints/Interactibles/DT_InstantPossessed.DT_InstantPossessed" (Variables|Default|GetName))
    (:then
      (Components|StaticMesh|SetStaticMesh _body (.Body (Utilities|Struct|BreakST_InstantPossessed _returnvalue)))
      (Rendering|Material|SetMaterial _body 0 (.Material (Utilities|Struct|BreakST_InstantPossessed _returnvalue)))
      (Rendering|Material|SetOverlayMaterial (Variables|Default|GetBody) "/Game/GA/VFX/Materials/MI_Outline_Blue.MI_Outline_Blue" :!class /Script/Engine.MeshComponent))))

(fn GetFearType
  (return (Variables|Default|GetFear%20Type)))

(fn GetFearAmount
  (return (Variables|Default|GetFear%20Amount)))

(fn IsUsed?
  (return (Variables|Default|GetIsUsed)))