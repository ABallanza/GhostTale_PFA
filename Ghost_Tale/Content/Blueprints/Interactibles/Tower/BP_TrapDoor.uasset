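; BP_TrapDoor is a tower trap interactible that, when activated, plays a hand animation and frightens the adventurer.
; Activate calls the parent, hides the tower mesh, then plays the trapped-door animation on the face A or B skeletal mesh according to Side.
; It then applies the configured fear type and amount to AdventurerRef through Effrayed.
; A separate Timeline macro provides gate-driven playback over a given length, unused by Activate.
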(event EventBeginPlay
  (|CallParentFunction) ; This node is disabled and will not be called.\nDrag off pins to build functionality.
)

(event Collision|EventActorBeginOverlap
  (params (OtherActor :type Actor%20Object%20Reference))
  (|CallParentFunction OtherActor) ; This node is disabled and will not be called.\nDrag off pins to build functionality.
)

(event EventTick
  (params (DeltaSeconds :type Float%20%28single-precision%29)))

(event EventActivate
  (params (BPAdventurer :type BP%20Adventurer%20Class%20Object%20Reference))
  (|CallParentFunction BPAdventurer)
  (if (Variables|Default|GetSide)
    (Rendering|SetVisibility (Variables|Default|GetTowerMesh) false true)
    ;[1 1 1] Fait l'animation face B
    (Components|SkeletalMesh|SetSkeletalMeshAsset (Variables|Default|GetNimationB) "/Game/GA/Meshes/Animation/Trapped_Door_Hand/AM_TrappedDoor_Hand.AM_TrappedDoor_Hand")
    (Components|Animation|PlayAnimation (Variables|Default|GetNimationB) "/Game/GA/Meshes/Animation/Trapped_Door_Hand/AM_TrappedDoor_Hand_Anim.AM_TrappedDoor_Hand_Anim" false)
    (else
      (Rendering|SetVisibility (Variables|Default|GetTowerMesh) false true)
      ;[1 1 1] Fait l'animation face A
      (Components|SkeletalMesh|SetSkeletalMeshAsset (Variables|Default|GetNimationA) "/Game/GA/Meshes/Animation/Trapped_Door_Hand/AM_TrappedDoor_Hand.AM_TrappedDoor_Hand")
      (Components|Animation|PlayAnimation (Variables|Default|GetNimationA) "/Game/GA/Meshes/Animation/Trapped_Door_Hand/AM_TrappedDoor_Hand_Anim.AM_TrappedDoor_Hand_Anim" false)))
  (Default|Effrayed (Variables|Default|GetAdventurer%20Ref) (Variables|Default|GetFearType) (Variables|Default|GetFearAmont)))

(fn ConstructionScript
  (|CallParentFunction))