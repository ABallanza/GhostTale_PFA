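; BP_CharacterSpawner is a level element that spawns the three playable-class characters: Wizard, Warrior and Thief.
; On BeginPlay it registers itself with BP_GameMode as CharacterSpawnerRef.
; Its SpawnCharacter event spawns each character at the world location of its own spawner component.
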(event Custom|Spawn%20Character
  (Game|SpawnActorfromClass "/Game/Blueprints/Characters/BP_Wizard.BP_Wizard_C" (Math|Transform|MakeTransform (Transformation|GetWorldLocation (Variables|Default|GetWizard%20Spawner)) "0, 0, 0" "1.000000,1.000000,1.000000") "Undefined" "MultiplyWithRoot" 0 20 0.1 0)
  (Game|SpawnActorfromClass "/Game/Blueprints/Characters/BP_Warrior.BP_Warrior_C" (Math|Transform|MakeTransform (Transformation|GetWorldLocation (Variables|Default|GetWarrior%20Spawner)) "0, 0, 0" "1.000000,1.000000,1.000000") "Undefined" "MultiplyWithRoot" 0 20 0.1 0)
  (Game|SpawnActorfromClass "/Game/Blueprints/Characters/BP_Thief.BP_Thief_C" (Math|Transform|MakeTransform (Transformation|GetWorldLocation (Variables|Default|GetThief%20Spawner)) "0, 0, 0" "1.000000,1.000000,1.000000") "Undefined" "MultiplyWithRoot" 0 20 0.1 0))

(event EventBeginPlay
  (bind _asbp_game_mode (Utilities|Casting|CastToBP_GameMode (Game|GetGameMode)))
  (Variables|/Game/Blueprints/BP_GameMode.BP_GameMode_C|SetCharacter%20Spawner%20Ref _asbp_game_mode self))

(fn ConstructionScript)