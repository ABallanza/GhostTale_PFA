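; BP_Room is a level element representing a room that groups linked doors and possessable objects, with a flag marking special rooms.
; On BeginPlay it registers itself with BP_GameMode and with each linked door and possessable.
; It exposes getters for that data and keeps a map of the possessable chosen for each adventurer, written and read through setter and lookup functions.
; ActivatePossessable is an empty stub.
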(event EventBeginPlay
  (bind _asbp_game_mode (Utilities|Casting|CastToBP_GameMode (Game|GetGameMode))
    (:then
      (bind _output_get (Variables|References|SetGameModeRef _asbp_game_mode))
      (Default|AddRoom _output_get self))
    (:CastFailed
      _))
  (for _array_element (Variables|References|GetLinkedDoors)
    (Default|AddRoom _array_element self))
  (for _array_element_2 (Variables|References|GetLinkedPossessables)
    (Default|SetRoom _array_element_2 self)))

(fn ConstructionScript)

(fn GetAllDoor
  (return (Variables|References|GetLinkedDoors)))

(fn GetIsSpecial
  (return (Variables|State|GetSpecial%20Room)))

(fn GetAllPossessables
  (return (Variables|References|GetLinkedPossessables)))

(fn ChoosePossessables
  (params (Adventurer :type BP%20Adventurer%20Class%20Object%20Reference))
  (bind _chosen_possessables (Variables|References|GetChosen%20Possessables))
  (bind (_value _returnvalue) (Utilities|Map|Find _chosen_possessables Adventurer))
  (if _returnvalue
    (return _value)
    (else
      (return 0))))

(fn ActivatePossessable
  (params (CurrentObjective :type BP%20Possessed%20Object%20Object%20Reference)))

(fn SetChosenPossessable
  (params (Adventurer :type BP%20Adventurer%20Class%20Object%20Reference) (Object :type BP%20Possessed%20Object%20Object%20Reference))
  (Utilities|Map|Add (Variables|References|GetChosen%20Possessables) Adventurer Object))