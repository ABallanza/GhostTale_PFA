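; BP_Door is a level door that links rooms and holds trapped, visited, close and impasse status flags.
; On BeginPlay it registers itself with BP_GameMode, and AddRoom fills its list of linked rooms.
; Getters expose the flags, and SetIsVisited updates the visited state.
; CheckIsImpasse indexes into the linked rooms relative to the current room and flags an impasse if that room has only one door.
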(event EventBeginPlay
  (bind _asbp_game_mode (Utilities|Casting|CastToBP_GameMode (Game|GetGameMode)))
  (bind _output_get (Variables|References|SetGameModeRef _asbp_game_mode))
  (Default|AddDoor _output_get self))

(fn ConstructionScript)

(fn AddRoom
  (params (Room :type BP%20Room%20Object%20Reference))
  (Utilities|Array|Add (Variables|References|GetLinkedRooms) Room))

(fn GetStatus
  (return (Variables|Status|GetIsTrapped) (Variables|Status|GetIs%20Visited) (Variables|Status|GetIs%20Close) (Variables|Status|GetIs%20Impasse)))

(fn GetIsTrapped
  (return (Variables|Status|GetIsTrapped)))

(fn GetIsVisited
  (return (Variables|Status|GetIs%20Visited)))

(fn GetIsClose
  (return (Variables|Status|GetIs%20Close)))

(fn GetIsImpasse
  (return (Variables|Status|GetIs%20Impasse)))

(fn CheckIsImpasse
  (params (Current%20Room :type BP%20Room%20Object%20Reference))
  (bind _linkedrooms (Variables|References|GetLinkedRooms))
  (bind _linkedrooms_2 (Variables|References|GetLinkedRooms))
  (bind _returnvalue (Utilities|Array|FindItem _linkedrooms_2 Current%20Room))
  (if (== -1 _returnvalue)
    (Development|PrintString "Error Check Impasse" true true "(R=1.000000,G=0.033939,B=0.000000,A=1.000000)" 1.2e+02)
    (return false)
    (elif (== (Utilities|Array|Length (Default|GetAllDoor (Utilities|Array|Get(acopy) _linkedrooms (Utilities|Operators|Subtract (Utilities|Array|Length _linkedrooms) _returnvalue -1)))) 1)
      (bind _output_get (Variables|Status|SetIs%20Impasse true))
      (return _output_get)
      (else
        (bind _output_get_2 (Variables|Status|SetIs%20Impasse false))
        (return _output_get_2)))))

(fn SetIsVisited
  (params (Value :type Boolean))
  (Variables|Status|SetIs%20Visited Value)
  (return))