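; Player controller that sets up the main HUD and routes Enhanced Input to the camera pawn and its build and cast parts.
; Game state decides the target: Setup drives trap building through BPBueld, Raid drives spell casting through BPCast.
; Entering or quitting either mode adds or removes its mapping context, tracked in an active list passed to the pause menu.
; Zoom is blocked while build mode is active.
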(event Custom|GetInteractUi
  (params (UI%20Interact :type WBP%20Possessed%20Object%20Object%20Reference))
  ;[0 0 0] Old
  (Utilities|IsValid (Variables|Default|GetUI%20Interact)
    (:Is%20Valid
      (Default|Delete (Variables|Default|GetUI%20Interact)))
    (:Is%20Not%20Valid
      _))
  (Variables|Default|SetUI%20Interact UI%20Interact))

(event Custom|ctrl%20release
  (bind _ui_interact (Variables|Default|GetUI%20Interact))
  ;[0 0 0] Old
  (switch Utilities|FlowControl|Switch|SwitchonE_GameState (Variables|/Game/Blueprints/BP_GameMode.BP_GameMode_C|GetE_GameState (Variables|Default|GetGame%20Mode%20Ref))
    (:NewEnumerator1
      (Default|MouseRClick (Variables|/Game/Blueprints/Camera/BP_CameraActor.BP_CameraActor_C|GetBP_Bueld (Variables|Default|GetCamera_Ref))))
    (:NewEnumerator2
      (Default|MouseRClick (Variables|/Game/Blueprints/Camera/BP_CameraActor.BP_CameraActor_C|GetBP_Cast (Variables|Default|GetCamera_Ref)))
      (Utilities|IsValid _ui_interact
        (:Is%20Valid
          (Default|Delete _ui_interact))))))

(event Custom|Quit%20Build%20Mode
  (params (Is%20Cast :type Boolean))
  (bind _ui_interact (Variables|Default|GetUI%20Interact))
  (if Is%20Cast
    (Default|MouseRClick (Variables|/Game/Blueprints/Camera/BP_CameraActor.BP_CameraActor_C|GetBP_Cast (Variables|Default|GetCamera_Ref)))
    (Utilities|IsValid _ui_interact
      (:Is%20Valid
        (Default|Delete _ui_interact))
      (:Is%20Not%20Valid
        _))
    (CallFunction|Add/RemoveMappingContext true "/Game/Blueprints/Controls/IMC_SpellMode.IMC_SpellMode")
    (else
      (Default|MouseRClick (Variables|/Game/Blueprints/Camera/BP_CameraActor.BP_CameraActor_C|GetBP_Bueld (Variables|Default|GetCamera_Ref)))
      (CallFunction|Add/RemoveMappingContext true "/Game/Blueprints/Controls/IMC_TrapMode.IMC_TrapMode"))))

(event Input|EnhancedActionEvents|EnhancedInputActionIA_SwitchSpell
  (params (ActionValue :type Float%20%28double-precision%29) (ElapsedSeconds :type Float%20%28double-precision%29) (TriggeredSeconds :type Float%20%28double-precision%29) (InputAction :type Input%20Action%20Object%20Reference :default "/Game/Blueprints/Controls/Spell/IA_SwitchSpell.IA_SwitchSpell"))
  (bind _camera_ref (Variables|Default|GetCamera_Ref))
  (bind _bp_cast (Variables|/Game/Blueprints/Camera/BP_CameraActor.BP_CameraActor_C|GetBP_Cast _camera_ref))
  ;[0 0.03858 1 0.6] Spell
  (Development|PrintString "SWITCHING SPELL")
  (if (> ActionValue 0.0)
    (Default|MWU _bp_cast)
    (else
      (Default|MWD _bp_cast))))

(event Input|EnhancedActionEvents|EnhancedInputActionIA_MouseClick
  (params (ActionValue :type Boolean) (ElapsedSeconds :type Float%20%28double-precision%29) (TriggeredSeconds :type Float%20%28double-precision%29) (InputAction :type Input%20Action%20Object%20Reference :default "/Game/Blueprints/Controls/Old/IA_MouseClick.IA_MouseClick"))
  ;[0 0 0] Old
  (:Started
    (Default|MouseClick (Variables|Default|GetCamera_Ref))
    (switch Utilities|FlowControl|Switch|SwitchonE_GameState (Variables|/Game/Blueprints/BP_GameMode.BP_GameMode_C|GetE_GameState (Variables|Default|GetGame%20Mode%20Ref))
      (:NewEnumerator1
        (Default|MouseClick (Variables|/Game/Blueprints/Camera/BP_CameraActor.BP_CameraActor_C|GetBP_Bueld (Variables|Default|GetCamera_Ref))))
      (:NewEnumerator2
        (Default|MouseClick (Variables|/Game/Blueprints/Camera/BP_CameraActor.BP_CameraActor_C|GetBP_Cast (Variables|Default|GetCamera_Ref)))))))

(event Input|EnhancedActionEvents|EnhancedInputActionIA_ZoomCamera
  (params (ActionValue :type Float%20%28double-precision%29) (ElapsedSeconds :type Float%20%28double-precision%29) (TriggeredSeconds :type Float%20%28double-precision%29) (InputAction :type Input%20Action%20Object%20Reference :default "/Game/Blueprints/Controls/Camera/IA_ZoomCamera.IA_ZoomCamera"))
  (bind _camera_ref (Variables|Default|GetCamera_Ref))
  (bind _camera_ref_2 (Variables|Default|GetCamera_Ref))
  ;[0.1146 0.1146 0.1146 0.7] Camera
  (if (not (or (Variables|/Game/Blueprints/Utilities/BP_Cast.BP_Cast_C|GetBuildMode (Variables|/Game/Blueprints/Camera/BP_CameraActor.BP_CameraActor_C|GetBP_Cast _camera_ref)) (Variables|/Game/Blueprints/Utilities/BP_Bueld.BP_Bueld_C|GetBuildMode (Variables|/Game/Blueprints/Camera/BP_CameraActor.BP_CameraActor_C|GetBP_Bueld _camera_ref))))
    (if (> ActionValue 0.0)
      (Default|MWU _camera_ref_2)
      (else
        (Default|MWD _camera_ref_2)))))

(event Input|EnhancedActionEvents|EnhancedInputActionIA_CastSpell
  (params (ActionValue :type Boolean) (ElapsedSeconds :type Float%20%28double-precision%29) (TriggeredSeconds :type Float%20%28double-precision%29) (InputAction :type Input%20Action%20Object%20Reference :default "/Game/Blueprints/Controls/Spell/IA_CastSpell.IA_CastSpell"))
  ;[0 0.03858 1 0.6] Spell
  (:Completed
    (Default|MouseClick (Variables|Default|GetCamera_Ref))
    (Default|MouseClick (Variables|/Game/Blueprints/Camera/BP_CameraActor.BP_CameraActor_C|GetBP_Cast (Variables|Default|GetCamera_Ref)))
    (CallFunction|QuitBuildMode true)))

(event Input|EnhancedActionEvents|EnhancedInputActionIA_SwitchBuild
  (params (ActionValue :type Float%20%28double-precision%29) (ElapsedSeconds :type Float%20%28double-precision%29) (TriggeredSeconds :type Float%20%28double-precision%29) (InputAction :type Input%20Action%20Object%20Reference :default "/Game/Blueprints/Controls/Trap/IA_SwitchBuild.IA_SwitchBuild"))
  (bind _camera_ref (Variables|Default|GetCamera_Ref))
  (bind _bp_bueld (Variables|/Game/Blueprints/Camera/BP_CameraActor.BP_CameraActor_C|GetBP_Bueld _camera_ref))
  ;[1 0 0.1784 0.8] Traps
  (Development|PrintString "SWITCHING TRAP")
  (if (> ActionValue 0.0)
    (Default|MWU _bp_bueld)
    (else
      (Default|MWD _bp_bueld))))

(event Input|EnhancedActionEvents|EnhancedInputActionIA_BuildTrap
  (params (ActionValue :type Boolean) (ElapsedSeconds :type Float%20%28double-precision%29) (TriggeredSeconds :type Float%20%28double-precision%29) (InputAction :type Input%20Action%20Object%20Reference :default "/Game/Blueprints/Controls/Trap/IA_BuildTrap.IA_BuildTrap"))
  ;[1 0 0.1784 0.8] Traps
  (:Completed
    (Default|MouseClick (Variables|Default|GetCamera_Ref))
    (Default|MouseClick (Variables|/Game/Blueprints/Camera/BP_CameraActor.BP_CameraActor_C|GetBP_Bueld (Variables|Default|GetCamera_Ref)))))

(event Input|EnhancedActionEvents|EnhancedInputActionIA_QuitTrapMode
  (params (ActionValue :type Boolean) (ElapsedSeconds :type Float%20%28double-precision%29) (TriggeredSeconds :type Float%20%28double-precision%29) (InputAction :type Input%20Action%20Object%20Reference :default "/Game/Blueprints/Controls/Trap/IA_QuitTrapMode.IA_QuitTrapMode"))
  ;[1 0 0.1784 0.8] Traps
  (:Completed
    (CallFunction|QuitBuildMode false)))

(event Input|EnhancedActionEvents|EnhancedInputActionIA_OpenBuildMode
  (params (ActionValue :type Boolean) (ElapsedSeconds :type Float%20%28double-precision%29) (TriggeredSeconds :type Float%20%28double-precision%29) (InputAction :type Input%20Action%20Object%20Reference :default "/Game/Blueprints/Controls/Main/IA_OpenBuildMode.IA_OpenBuildMode"))
  (bind _camera_ref (Variables|Default|GetCamera_Ref))
  ;[0.06765 0.9901 1] Main
  (:Completed
    (if (or (Variables|/Game/Blueprints/Utilities/BP_Cast.BP_Cast_C|GetBuildMode (Variables|/Game/Blueprints/Camera/BP_CameraActor.BP_CameraActor_C|GetBP_Cast _camera_ref)) (Variables|/Game/Blueprints/Utilities/BP_Bueld.BP_Bueld_C|GetBuildMode (Variables|/Game/Blueprints/Camera/BP_CameraActor.BP_CameraActor_C|GetBP_Bueld _camera_ref)))
      (CallFunction|QuitBuildMode (Variables|/Game/Blueprints/Utilities/BP_Cast.BP_Cast_C|GetBuildMode (Variables|/Game/Blueprints/Camera/BP_CameraActor.BP_CameraActor_C|GetBP_Cast (Variables|Default|GetCamera_Ref))))
      (else
        (switch Utilities|FlowControl|Switch|SwitchonE_GameState (Variables|/Game/Blueprints/BP_GameMode.BP_GameMode_C|GetE_GameState (Variables|Default|GetGame%20Mode%20Ref))
          (:NewEnumerator1
            (Default|Build (Variables|/Game/Blueprints/Camera/BP_CameraActor.BP_CameraActor_C|GetBP_Bueld (Variables|Default|GetCamera_Ref)))
            (CallFunction|Add/RemoveMappingContext false "/Game/Blueprints/Controls/IMC_TrapMode.IMC_TrapMode"))
          (:NewEnumerator2
            (Default|Build (Variables|/Game/Blueprints/Camera/BP_CameraActor.BP_CameraActor_C|GetBP_Cast (Variables|Default|GetCamera_Ref)))
            (CallFunction|Add/RemoveMappingContext false "/Game/Blueprints/Controls/IMC_SpellMode.IMC_SpellMode")))))))

(event Input|EnhancedActionEvents|EnhancedInputActionIA_Pause
  (params (ActionValue :type Boolean) (ElapsedSeconds :type Float%20%28double-precision%29) (TriggeredSeconds :type Float%20%28double-precision%29) (InputAction :type Input%20Action%20Object%20Reference :default "/Game/Blueprints/Controls/Main/IA_Pause.IA_Pause"))
  ;[0.06765 0.9901 1] Main
  (:Started
    (Default|OpenPauseMenu (Variables|Default|GetGame%20Mode%20Ref) (Variables|Default|GetActiveMappingContext))))

(event Input|EnhancedActionEvents|EnhancedInputActionIA_QuitMenu
  (params (ActionValue :type Boolean) (ElapsedSeconds :type Float%20%28double-precision%29) (TriggeredSeconds :type Float%20%28double-precision%29) (InputAction :type Input%20Action%20Object%20Reference :default "/Game/Blueprints/Controls/Menu/IA_QuitMenu.IA_QuitMenu"))
  ;[1 0.6703 0] Menu
  (Default|QuitPauseMenu (Variables|Default|GetGame%20Mode%20Ref)))

(event Input|EnhancedActionEvents|EnhancedInputActionIA_WheelDown
  (params (ActionValue :type Boolean) (ElapsedSeconds :type Float%20%28double-precision%29) (TriggeredSeconds :type Float%20%28double-precision%29) (InputAction :type Input%20Action%20Object%20Reference :default "/Game/Blueprints/Controls/Old/IA_WheelDown.IA_WheelDown"))
  ;[0 0 0] Old
  (if (Variables|Default|GetCanPlace)
    (switch Utilities|FlowControl|Switch|SwitchonE_GameState (Variables|/Game/Blueprints/BP_GameMode.BP_GameMode_C|GetE_GameState (Variables|Default|GetGame%20Mode%20Ref))
      (:NewEnumerator1
        (Default|MWD (Variables|/Game/Blueprints/Camera/BP_CameraActor.BP_CameraActor_C|GetBP_Bueld (Variables|Default|GetCamera_Ref))))
      (:NewEnumerator2))))

(event Input|EnhancedActionEvents|EnhancedInputActionIA_Navigation
  (params (ActionValue :type Vector%202D%20Structure) (ElapsedSeconds :type Float%20%28double-precision%29) (TriggeredSeconds :type Float%20%28double-precision%29) (InputAction :type Input%20Action%20Object%20Reference :default "/Game/Blueprints/Controls/Menu/IA_Navigation.IA_Navigation"))
  ;[1 0.6703 0] Menu
)

(event Input|EnhancedActionEvents|EnhancedInputActionIA_Enter
  (params (ActionValue :type Boolean) (ElapsedSeconds :type Float%20%28double-precision%29) (TriggeredSeconds :type Float%20%28double-precision%29) (InputAction :type Input%20Action%20Object%20Reference :default "/Game/Blueprints/Controls/Menu/IA_Enter.IA_Enter"))
  ;[1 0.6703 0] Menu
)

(event Input|EnhancedActionEvents|EnhancedInputActionIA_Build
  (params (ActionValue :type Boolean) (ElapsedSeconds :type Float%20%28double-precision%29) (TriggeredSeconds :type Float%20%28double-precision%29) (InputAction :type Input%20Action%20Object%20Reference :default "/Game/Blueprints/Controls/Old/IA_Build.IA_Build"))
  ;[0 0 0] Old
  (:Started
    (switch Utilities|FlowControl|Switch|SwitchonE_GameState (Variables|/Game/Blueprints/BP_GameMode.BP_GameMode_C|GetE_GameState (Variables|Default|GetGame%20Mode%20Ref))
      (:NewEnumerator1
        (Default|Build (Variables|/Game/Blueprints/Camera/BP_CameraActor.BP_CameraActor_C|GetBP_Bueld (Variables|Default|GetCamera_Ref))))
      (:NewEnumerator2
        (Default|Build (Variables|/Game/Blueprints/Camera/BP_CameraActor.BP_CameraActor_C|GetBP_Cast (Variables|Default|GetCamera_Ref)))))))

(event Input|EnhancedActionEvents|EnhancedInputActionIA_WheelUp
  (params (ActionValue :type Boolean) (ElapsedSeconds :type Float%20%28double-precision%29) (TriggeredSeconds :type Float%20%28double-precision%29) (InputAction :type Input%20Action%20Object%20Reference :default "/Game/Blueprints/Controls/Old/IA_WheelUp.IA_WheelUp"))
  ;[0 0 0] Old
  (if (Variables|Default|GetCanPlace)
    (switch Utilities|FlowControl|Switch|SwitchonE_GameState (Variables|/Game/Blueprints/BP_GameMode.BP_GameMode_C|GetE_GameState (Variables|Default|GetGame%20Mode%20Ref))
      (:NewEnumerator1
        (Default|MWU (Variables|/Game/Blueprints/Camera/BP_CameraActor.BP_CameraActor_C|GetBP_Bueld (Variables|Default|GetCamera_Ref))))
      (:NewEnumerator2))))

(event Input|EnhancedActionEvents|EnhancedInputActionIA_RightClick
  (params (ActionValue :type Boolean) (ElapsedSeconds :type Float%20%28double-precision%29) (TriggeredSeconds :type Float%20%28double-precision%29) (InputAction :type Input%20Action%20Object%20Reference :default "/Game/Blueprints/Controls/Old/IA_RightClick.IA_RightClick"))
  (bind _ui_interact (Variables|Default|GetUI%20Interact))
  ;[0 0 0] Old
  (switch Utilities|FlowControl|Switch|SwitchonE_GameState (Variables|/Game/Blueprints/BP_GameMode.BP_GameMode_C|GetE_GameState (Variables|Default|GetGame%20Mode%20Ref))
    (:NewEnumerator1
      (Default|MouseRClick (Variables|/Game/Blueprints/Camera/BP_CameraActor.BP_CameraActor_C|GetBP_Bueld (Variables|Default|GetCamera_Ref))))
    (:NewEnumerator2
      (Default|MouseRClick (Variables|/Game/Blueprints/Camera/BP_CameraActor.BP_CameraActor_C|GetBP_Cast (Variables|Default|GetCamera_Ref)))
      (Utilities|IsValid _ui_interact
        (:Is%20Valid
          (Default|Delete _ui_interact))))))

(event Input|EnhancedActionEvents|EnhancedInputActionIA_MoveCamera
  (params (ActionValue :type Vector%202D%20Structure) (ElapsedSeconds :type Float%20%28double-precision%29) (TriggeredSeconds :type Float%20%28double-precision%29) (InputAction :type Input%20Action%20Object%20Reference :default "/Game/Blueprints/Controls/Camera/IA_MoveCamera.IA_MoveCamera"))
  ;[0.1146 0.1146 0.1146 0.7] Camera
  (Default|MoveCamera (Variables|Default|GetCamera_Ref) ActionValue))

(event Input|EnhancedActionEvents|EnhancedInputActionIA_QuitSpellMode
  (params (ActionValue :type Boolean) (ElapsedSeconds :type Float%20%28double-precision%29) (TriggeredSeconds :type Float%20%28double-precision%29) (InputAction :type Input%20Action%20Object%20Reference :default "/Game/Blueprints/Controls/Spell/IA_QuitSpellMode.IA_QuitSpellMode"))
  ;[0 0.03858 1 0.6] Spell
  (CallFunction|QuitBuildMode true))

(event Input|EnhancedActionEvents|EnhancedInputActionIA_AllowingPlacement
  (params (ActionValue :type Boolean) (ElapsedSeconds :type Float%20%28double-precision%29) (TriggeredSeconds :type Float%20%28double-precision%29) (InputAction :type Input%20Action%20Object%20Reference :default "/Game/Blueprints/Controls/Old/IA_AllowingPlacement.IA_AllowingPlacement"))
  ;[0 0 0] Old
  (:Triggered
    (Variables|Default|SetCanPlace ActionValue :!label _label))
  (:Completed
    (CallFunction|CtrlRelease)
    (goto _label)))

(event Input|EnhancedActionEvents|EnhancedInputActionIA_RotateCamera
  (params (ActionValue :type Vector%202D%20Structure) (ElapsedSeconds :type Float%20%28double-precision%29) (TriggeredSeconds :type Float%20%28double-precision%29) (InputAction :type Input%20Action%20Object%20Reference :default "/Game/Blueprints/Controls/Camera/IA_RotateCamera.IA_RotateCamera"))
  ;[0.1146 0.1146 0.1146 0.7] Camera
  (Default|RotateCamera (Variables|Default|GetCamera_Ref) ActionValue))

(event EventBeginPlay
  ;[1 1 1] Event Begin Play
  (CallFunction|Add/RemoveMappingContext false "/Game/Blueprints/Controls/IMC_Main.IMC_Main")
  (CallFunction|Add/RemoveMappingContext false "/Game/Blueprints/Controls/IMC_Camera.IMC_Camera")
  (CallFunction|Add/RemoveMappingContext false "/Game/Blueprints/Controls/IMC_Test.IMC_Test")
  (bind _asbp_game_mode (Utilities|Casting|CastToBP_GameMode (Game|GetGameMode)))
  (bind _output_get (Variables|Default|SetGame%20Mode%20Ref _asbp_game_mode))
  (bind _returnvalue (UserInterface|CreateWidget "/Game/Blueprints/GUI/WBP_Main.WBP_Main_C" self _output_get))
  (bind _output_get_2 (Variables|Default|SetMain_WBP _returnvalue))
  (UserInterface|Viewport|AddtoViewport _output_get_2 0)
  (Default|SetMainWidget _output_get (Variables|Default|GetMain_WBP))
  (Default|GetWidgetRef (Variables|/Game/Blueprints/Camera/BP_CameraActor.BP_CameraActor_C|GetBP_Bueld (Variables|Default|GetCamera_Ref)) (Variables|Default|GetMain_WBP))
  (Default|GetWidgetRef (Variables|/Game/Blueprints/Camera/BP_CameraActor.BP_CameraActor_C|GetBP_Cast (Variables|Default|GetCamera_Ref)) (Variables|Default|GetMain_WBP)))

(fn ConstructionScript)

(fn Add/RemoveMappingContext
  (params (Remove :type Boolean) (Target%20Context :type Input%20Mapping%20Context%20Object%20Reference))
  (bind _returnvalue (PlayerController|LocalPlayerSubsystems|GetEnhancedInputLocalPlayerSubsystem))
  (bind _activemappingcontext (Variables|Default|GetActiveMappingContext))
  (LocalVariables|SetTarget%20Mapping Target%20Context)
  (Utilities|IsValid _returnvalue
    (:Is%20Valid
      (if Remove
        (Input|RemoveMappingContext _returnvalue (LocalVariables|GetTarget%20Mapping) "(bIgnoreAllPressedKeysUntilRelease=True,bForceImmediately=False,bNotifyUserSettings=False)")
        (Utilities|Array|RemoveItem _activemappingcontext (LocalVariables|GetTarget%20Mapping))
        (else
          (Input|AddMappingContext _returnvalue (LocalVariables|GetTarget%20Mapping) 0 "(bIgnoreAllPressedKeysUntilRelease=True,bForceImmediately=False,bNotifyUserSettings=False)")
          (Utilities|Array|Add _activemappingcontext (LocalVariables|GetTarget%20Mapping)))))
    (:Is%20Not%20Valid
      (Development|PrintText "Mapping Invalid" true true "(R=0.811572,G=0.210169,B=1.000000,A=1.000000)" 2.5e+03))))

(fn GetActiveMapping
  (return (Variables|Default|GetActiveMappingContext)))