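; Adventurer character class with a fear system: scares fill a fear gauge that sets a discrete fear level.
; Scare types are checked against phobia and immunity lists to choose a multiplier; the reaction handler is still empty.
; Each tick the gauge decays toward the current level's threshold, computed at construction, and the overhead fear bar turns to face the camera.
; It also records passed doors.
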(event Custom|Effrayed
  (params (Type :type E_Fear%20Enum :default "NewEnumerator4") (Amont :type Float%20%28double-precision%29))
  ;[0.04369 0.1094 1 0.3] Fear System
  ;;[0.05007 0.779 1 0.8] Quand les aventuriers sont effrayés
  (bind (_reaction _multiplyer) (CallFunction|FearReaction Type))
  (CallFunction|FearReaction _reaction)
  (Default|ChangeGauge (Variables|FearSystem|GetFearGauge) 0.0 false (* _multiplyer Amont))
  (bind _current_level (CallFunction|SetFearLevel))
  (Variables|FearSystem|SetCurrent%20Fear%20Level _current_level))

(event Custom|Reassured
  ;[0.04369 0.1094 1 0.3] Fear System
  ;;[0.2188 0.1005 1] Diminution de la peur avec le temps
  (bind _reassurence_value (CallFunction|SetReassurence))
  (Default|ChangeGauge (Variables|FearSystem|GetFearGauge) 0.0 true _reassurence_value))

(event Custom|Fear%20Reaction
  (params (Reaction :type E_Reaction%20Enum :default "NewEnumerator0"))
  ;[0.04369 0.1094 1 0.3] Fear System
  (switch Utilities|FlowControl|Switch|SwitchonE_Reaction Reaction))

(event Custom|Begining%20Setter
  ;[1 1 1 0.4] Event Begin Play
  ;;[0.4323 0.4323 0.4323 0.8] Set correctement tous les paramètres quand on lance le jeu
  (bind _aswbp_fear_bar (Utilities|Casting|CastToWBP_FearBar (UserInterface|GetWidget (Variables|Widget|GetFearBarWidget))))
  (bind _output_get (Variables|Widget|SetWidget%20Ref _aswbp_fear_bar))
  (Variables|/Game/Blueprints/GUI/WBP_FearBar.WBP_FearBar_C|SetOwner _output_get self)
  (bind _current_level (CallFunction|SetFearLevel))
  (Variables|FearSystem|SetCurrent%20Fear%20Level _current_level)
  (bind _asbp_camera_controller (Utilities|Casting|CastToBP_CameraController (Game|GetPlayerController 0)))
  (Variables|Widget|SetCamera%20Ref (Variables|/Game/Blueprints/Controls/BP_CameraController.BP_CameraController_C|GetCamera_Ref _asbp_camera_controller)))

(event Custom|WidgetOnCamera
  (bind _fearbarwidget (Variables|Widget|GetFearBarWidget))
  ;[0 0.06516 1 0.3] Gestion des Widgets
  ;;[0.1884 0 1 0.8] Rotation de la bar de peur vers la caméra
  (Transformation|SetWorldRotation _fearbarwidget (Math|Rotator|FindLookatRotation (Transformation|GetWorldLocation _fearbarwidget) (Transformation|GetActorLocation (Variables|Widget|GetCamera%20Ref))) false false))

(event EventBeginPlay
  ;[1 1 1 0.4] Event Begin Play
  (CallFunction|BeginingSetter))

(event EventTick
  (params (DeltaSeconds :type Float%20%28single-precision%29))
  ;[0.276 0.1536 0] Debug
  ;;[0.9878 1 0.008979] Event Tick
  (CallFunction|Reassured)
  (CallFunction|WidgetonCamera))

(fn ConstructionScript
  (LocalVariables|SetFearLevelStep (/ (Default|GetMaxGauge (Variables|FearSystem|GetFearGauge)) (Variables|FearSystem|GetMax%20Fear%20Level)))
  (for _index (range 1 (Variables|FearSystem|GetMax%20Fear%20Level))
    (Utilities|Array|Add (Variables|FearSystem|GetFearLevelSteps) (* _index (LocalVariables|GetFearLevelStep)))))

(fn FearReaction
  (params (Fear :type E_Fear%20Enum :default "NewEnumerator4"))
  (if (== (Utilities|Array|FindItem (Variables|FearSystem|GetPhobia) Fear) -1)
    (if (== (Utilities|Array|FindItem (Variables|FearSystem|GetImunity) Fear) -1)
      (LocalVariables|SetReactionType "NewEnumerator2")
      (else
        (LocalVariables|SetReactionType "NewEnumerator0")))
    (else
      (LocalVariables|SetReactionType "NewEnumerator4")))
  (return (LocalVariables|GetReactionType) (.Value (Utilities|Map|Find (Variables|FearSystem|GetFear%20Multiplyer) (LocalVariables|GetReactionType)))))

(fn SetFearLevel
  (for _index (range 0 (- (Variables|FearSystem|GetMax%20Fear%20Level) 1))
    (if (<= (Utilities|Array|Get(acopy) (Variables|FearSystem|GetFearLevelSteps) _index) (Default|GetCurrentGauge (Variables|FearSystem|GetFearGauge)))
      (Math|Integer|IncrementInt (LocalVariables|GetLevelCounter))))
  (return (LocalVariables|GetLevelCounter)))

(fn SetReassurence
  (LocalVariables|SetFear%20Step (Utilities|Array|Get(acopy) (Variables|FearSystem|GetFearLevelSteps) (- (Variables|FearSystem|GetCurrent%20Fear%20Level) 1)))
  (if (<= (- (Default|GetCurrentGauge (Variables|FearSystem|GetFearGauge)) (Variables|FearSystem|GetReassurence%20Speed)) (LocalVariables|GetFear%20Step))
    (return (- (Default|GetCurrentGauge (Variables|FearSystem|GetFearGauge)) (LocalVariables|GetFear%20Step)))
    (else
      (return (Variables|FearSystem|GetReassurence%20Speed)))))

(fn AddPassedDoor
  (params (Door :type BP%20Door%20Object%20Reference))
  (Utilities|Array|Add (Variables|Path|GetPassedDoors) Door))