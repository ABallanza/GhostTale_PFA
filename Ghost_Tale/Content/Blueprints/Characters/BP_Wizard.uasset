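; BP_Wizard is the Wizard adventurer character, an AI-driven party member that runs the BT_Leader behavior tree.
; On BeginPlay it registers with BP_GameMode, caches its AI controller, and activates the tree after a short delay.
; It then fetches Thief and Warrior references from the game mode.
; An unused debug event retries until it can write a BP_Room into the blackboard's CurrentRoom key.
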(event Custom|Know%20Others%20Characters
  (bind _game_mode_ref (Variables|References|GetGame%20Mode%20Ref))
  (Variables|References|SetThiefREF (Default|GetThief _game_mode_ref))
  (Variables|References|SetWarriorREF (Default|GetWarrior _game_mode_ref))
  (Development|PrintString "Adventurer Ready To Go"))

(event Custom|DebugRoom
  ;[1 0 0] DEBUG
  (bind _returnvalue (Actor|GetActorOfClass "/Game/Blueprints/LevelElements/BP_Room.BP_Room_C"))
  (Utilities|IsValid _returnvalue
    (:Is%20Valid
      (AI|Components|Blackboard|SetValueasObject (Variables|/Script/AIModule.AIController|GetBlackboard (Variables|References|GetAI%20Controller%20Ref)) (Utilities|Name|MakeLiteralName "CurrentRoom") _returnvalue)
      (Development|PrintString "DONE"))
    (:Is%20Not%20Valid
      (CallFunction|DebugRoom))))

(event EventBeginPlay
  (|CallParentFunction)
  (bind _asbp_game_mode (Utilities|Casting|CastToBP_GameMode (Game|GetGameMode)))
  (bind _output_get (Variables|References|SetGame%20Mode%20Ref _asbp_game_mode))
  (Default|AddWizard _output_get self)
  (bind _asai_controller (Utilities|Casting|CastToAI_Controller (Pawn|GetController)))
  (Variables|References|SetAI%20Controller%20Ref _asai_controller)
  (Utilities|FlowControl|Delay 0.5)
  (Variables|Default|SetBehaviorTree "/Game/Blueprints/Characters/AI/BT_Leader.BT_Leader")
  (CallFunction|ActivateBehaviorTree)
  (CallFunction|KnowOthersCharacters))

(fn ConstructionScript
  (|CallParentFunction))