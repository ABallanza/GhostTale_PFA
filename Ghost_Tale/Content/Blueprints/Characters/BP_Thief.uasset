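; BP_Thief is the Thief character, which registers itself with BP_GameMode and is driven by the BT_Follower behavior tree.
; On BeginPlay it adds itself to the game mode, waits briefly, then has its AI_Controller run the tree.
; It then caches Wizard and Warrior references from the game mode, with the short delay preceding both the controller cast and these lookups.
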(event Custom|Know%20Others%20Characters
  (bind _game_mode_ref (Variables|References|GetGame%20Mode%20Ref))
  (Variables|References|SetWizardREF (Default|GetWizard _game_mode_ref))
  (Variables|References|SetWarriorREF (Default|GetWarrior _game_mode_ref)))

(event EventBeginPlay
  (|CallParentFunction)
  (bind _asbp_game_mode (Utilities|Casting|CastToBP_GameMode (Game|GetGameMode)))
  (bind _output_get (Variables|References|SetGame%20Mode%20Ref _asbp_game_mode))
  (Default|AddThief _output_get self)
  (Utilities|FlowControl|Delay 0.2)
  (bind _asai_controller (Utilities|Casting|CastToAI_Controller (Pawn|GetController)))
  (bind _output_get_2 (Variables|References|SetAI%20Controller%20Ref _asai_controller))
  (AI|RunBehaviorTree _output_get_2 "/Game/Blueprints/Characters/AI/BT_Follower.BT_Follower")
  (CallFunction|KnowOthersCharacters))

(fn ConstructionScript
  (|CallParentFunction))