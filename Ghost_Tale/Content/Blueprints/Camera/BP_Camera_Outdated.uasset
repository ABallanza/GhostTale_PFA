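; Outdated player camera, likely for a tower-building game, that switches to flying movement and shows the mouse cursor on BeginPlay.
; ChangeColor gathers primitive siblings of a given component, caches each slot 0 material in a single variable, then sets that slot with no material specified.
; Cursor-trace detection of Tower-tagged actors outside build mode and directional movement logic are disconnected, leaving the IA_MoveCamera input event empty.
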(event Custom|ChangeColor
  (params (Component :type Scene%20Component%20Object%20Reference))
  (for _array_element (Components|GetChildrenComponents (Transformation|GetAttachParent Component) false)
    (bind _asprimitive_component (Utilities|Casting|CastToPrimitiveComponent _array_element))
    (Utilities|Array|Add (Variables|ChangeColor|GetCompList) _asprimitive_component))
  (Variables|ChangeColor|SetC_Comp (Variables|ChangeColor|GetCompList))
  (Utilities|Array|Clear (Variables|ChangeColor|GetCompList))
  (for _array_element_2 (Variables|ChangeColor|GetC_Comp)
    (Variables|ChangeColor|SetC_Comp_OriginalMaterial (Rendering|Material|GetMaterial _array_element_2 0))
    (Rendering|Material|SetMaterial _array_element_2 0 0)))

(event Input|EnhancedActionEvents|EnhancedInputActionIA_MoveCamera
  (params (ActionValue :type Vector%202D%20Structure) (ElapsedSeconds :type Float%20%28double-precision%29) (TriggeredSeconds :type Float%20%28double-precision%29) (InputAction :type Input%20Action%20Object%20Reference :default "/Game/Blueprints/Controls/IA_MoveCamera.IA_MoveCamera")))

(event Collision|EventActorBeginOverlap
  (params (OtherActor :type Actor%20Object%20Reference)))

(event EventBeginPlay
  (Pawn|Components|CharacterMovement|SetMovementMode (Variables|Character|GetCharacterMovement) "MOVE_Flying" 0)
  (Variables|/Script/Engine.PlayerController|SetbShowMouseCursor (Game|GetPlayerController 0) true))

(fn ConstructionScript)