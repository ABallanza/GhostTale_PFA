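; Player camera actor that pans, yaw-rotates, zooms and glides to focus on the Wizard.
; BeginPlay registers it with BP_CameraController, becomes the view target and traces forward to place the Frheg pivot, with Dayum as camera anchor.
; A custom DelayUntilNextTick timeline macro drives zoom and focus lerps, reversing into negative alpha for opposite zoom.
; The click trace for "Trap" actors takes no action on hits, and several offset chains are disconnected.
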(event Custom|MoveCamera
  (params (AxisValue :type Vector%202D%20Structure))
  (Variables|Default|SetAxis%20Value AxisValue)
  (Transformation|AddLocalOffset (Variables|Default|GetSceneComponent) (Math|Conversions|ToVector(Vector2D) (* (Variables|Default|GetAxis%20Value) (Variables|Default|GetSpeed))) false false))

(event Custom|Horizontal_Limite
  (Variables|Default|SetAxis%20Value (Math|Vector2D|MakeVector2D (.x (Math|Conversions|ToVector(Vector2D) (Variables|Default|GetAxis%20Value))) 0.0)))

(event Custom|MWU
  (bind _cameracomponent (Variables|CameraActor|GetCameraComponent))
  (bind _returnvalue (Transformation|GetWorldLocation _cameracomponent))
  ;[0 0.3761 1] Zoom
  (if (> (.z (Variables|/Script/Engine.SceneComponent|GetRelativeLocation (Variables|CameraActor|GetCameraComponent))) (Variables|Zoom|GetZoomMax))
    (bind _position (Utilities|Timeline 0.1) ; enters at Reverse
      (:Update
        (Transformation|SetWorldLocation _cameracomponent (Math|Vector|Lerp(Vector) _returnvalue (+ _returnvalue (* (- _returnvalue (Transformation|GetWorldLocation (Variables|Default|GetPointOfView))) (Variables|Zoom|GetZoomSpeed))) _position) false false))
      (:Finished
        (Transformation|SetWorldLocation (Variables|Default|GetDayum) (Transformation|GetWorldLocation (Variables|CameraActor|GetCameraComponent)) false false)))))

(event Custom|MouseClick
  (bind _returnvalue (Game|GetPlayerController 0))
  (bind (_worldlocation _worlddirection) (Game|Player|ConvertMouseLocationToWorldSpace _returnvalue))
  (if (not (Variables|/Game/Blueprints/Utilities/BP_Bueld.BP_Bueld_C|GetBuildMode (Variables|Default|GetBP_Bueld)))
    (bind (_outhit _returnvalue_2) (Collision|LineTraceByChannel _worldlocation (+ _worldlocation (* _worlddirection 2e+03)) "TraceTypeQuery1" false 0 "None"))
    (if _returnvalue_2
      (if (!= (Variables|Default|GetNew_Trap) (.HitActor (Collision|BreakHitResult _outhit)))
        (if (Actor|ActorHasTag (.HitActor (Collision|BreakHitResult _outhit)) "Trap")
          _)
        (else
          (Variables|Default|SetNew_Trap 0))))))

(event Custom|MWD
  (bind _cameracomponent (Variables|CameraActor|GetCameraComponent))
  (bind _returnvalue (Transformation|GetWorldLocation _cameracomponent))
  ;[0 0.3761 1] Zoom
  (if (< (.z (Variables|/Script/Engine.SceneComponent|GetRelativeLocation (Variables|CameraActor|GetCameraComponent))) (Variables|Zoom|GetZoomMin))
    (bind _position (Utilities|Timeline 0.1) ; enters at Play From Start
      (:Update
        (Transformation|SetWorldLocation _cameracomponent (Math|Vector|Lerp(Vector) _returnvalue (+ _returnvalue (* (- _returnvalue (Transformation|GetWorldLocation (Variables|Default|GetPointOfView))) (Variables|Zoom|GetZoomSpeed))) _position) false false))
      (:Finished
        (Transformation|SetWorldLocation (Variables|Default|GetDayum) (Transformation|GetWorldLocation (Variables|CameraActor|GetCameraComponent)) false false)))))

(event Custom|RotateCamera
  (params (Vector2D :type Vector%202D%20Structure))
  (Variables|Default|Setpositioning (Transformation|GetWorldLocation (Variables|Default|GetFrheg)))
  (Transformation|AddWorldRotation (Variables|Default|GetSceneComponent) (Math|Rotator|MakeRotator 0.0 0.0 (.x (* Vector2D (Variables|Default|GetRotateSpeed)))) false false)
  (Transformation|SetWorldLocation (Variables|Default|GetFrheg) (Variables|Default|Getpositioning) false false)
  (Transformation|SetWorldLocation (Variables|CameraActor|GetCameraComponent) (Transformation|GetWorldLocation (Variables|Default|GetDayum)) false false))

(event Custom|FocusCam
  (bind _as_bp_game_mode (Variables|Default|GetAs%20BP%20Game%20Mode))
  (bind _wizard_ref (Default|GetWizard _as_bp_game_mode))
  ;[1 0.6958 0] Focus Adventurer
  (if (not (Variables|Default|GetNimationInProgress))
    (Variables|Default|SetNimationInProgress true)
    (Utilities|IsValid _wizard_ref
      (:Is%20Valid
        (Transformation|SetWorldLocation (Variables|Default|GetFrheg) (Transformation|GetWorldLocation (Variables|/Script/Engine.Character|GetMesh _wizard_ref)) false false)
        (Variables|Default|Setpositioning (Transformation|GetWorldLocation (Variables|CameraActor|GetCameraComponent)))
        (bind _position (Utilities|Timeline 1.0) ; enters at Play From Start
          (:Update
            (Transformation|SetWorldLocation (Variables|CameraActor|GetCameraComponent) (Math|Vector|Lerp(Vector) (Variables|Default|Getpositioning) (Transformation|GetWorldLocation (Variables|Default|GetDayum)) _position) false false))
          (:Finished
            (Variables|Default|SetNimationInProgress false)))))))

(event EventBeginPlay
  (bind _cameracomponent (Variables|CameraActor|GetCameraComponent))
  (bind _returnvalue (Transformation|GetWorldLocation _cameracomponent))
  ;[1 1 1] EventBeginPlay
  (bind _asbp_game_mode (Utilities|Casting|CastToBP_GameMode (Game|GetGameMode)))
  (Variables|Default|SetAs%20BP%20Game%20Mode _asbp_game_mode)
  (bind _asbp_camera_controller (Utilities|Casting|CastToBP_CameraController (Game|GetPlayerController 0)))
  (Variables|/Game/Blueprints/Controls/BP_CameraController.BP_CameraController_C|SetCamera_Ref _asbp_camera_controller self)
  (Game|Player|SetViewTargetwithBlend (Game|GetPlayerController 0) self 0.0 "VTBlend_Linear" 0.0 false)
  (bind (_outhit _returnvalue_2) (Collision|LineTraceByChannel _returnvalue (+ _returnvalue (* (Math|Vector|GetForwardVector _cameracomponent) 4e+03)) "TraceTypeQuery1" false 0 "None"))
  (if _returnvalue_2
    (Variables|Default|Setpositioning (Transformation|GetWorldLocation (Variables|Default|GetDayum)))
    (Transformation|SetWorldLocation (Variables|Default|GetFrheg) (.Location (Collision|BreakHitResult _outhit)) false false)
    (Transformation|SetWorldLocation (Variables|Default|GetDayum) (Variables|Default|Getpositioning) false false)
    (Transformation|SetWorldLocation (Variables|CameraActor|GetCameraComponent) (Transformation|GetWorldLocation (Variables|Default|GetDayum)) false false)))

(fn ConstructionScript)