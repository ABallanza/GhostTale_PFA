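; Game mode for a dungeon-defense game, running the phase state machine from trap setup to adventurer raids.
; SetGameState drives music, tutorial text, light color, spellbook, character spawning and trap-zone visibility, alongside pause-menu input switching.
; It owns mana and cleanliness gauges: dirt and tidying set a multiplier that scales mana cost, and spent mana regenerates on Tick.
; Actor references are registered here; the setup countdown's startup is disconnected, and Ritual immediately requests EndGame.
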(event Custom|RaidBegin
  ;[1 1 1] Event Begin Play
  (Variables|GameState|SetE_GameState "NewEnumerator1")
  (CallFunction|PlayTrack)
  (CallFunction|SetGameState (Variables|GameState|GetE_GameState)))

(event Custom|Get%20BP_Cast%20Ref
  (params (BP_cast :type BP%20Cast%20Object%20Reference))
  ;[1 1 1] Event Begin Play
  (Variables|Default|SetBP_Cast BP_cast))

(event Custom|Begin%20Raid%20State
  ;[0 0.1094 0.02125 0.6] Game State
  (Default|SpawnCharacter (Variables|References|GetCharacter%20Spawner%20Ref))
  (Default|SwitchSpellBook (Variables|References|GetController%20Ref) true)
  (CallFunction|RLight)
  (CallFunction|HideTrapZone)
  (Default|TickDesactivation (Variables|/Game/Blueprints/Camera/BP_CameraActor.BP_CameraActor_C|GetBP_Clean (Variables|/Game/Blueprints/Controls/BP_CameraController.BP_CameraController_C|GetCamera_Ref (Variables|References|GetController%20Ref)))))

(event Custom|Open%20Pause%20Menu
  (params (Previous%20Mapping :type Array%20of%20Input%20Mapping%20Context%20Object%20References))
  (bind _controller_ref (Variables|References|GetController%20Ref))
  ;[0 0.1094 0.02125 0.6] Game State
  ;;[1 0 0.7648] Pause Menu
  (bind _output_get (Variables|Pause|SetPrevious%20Mapping%20%28Pause%29 Previous%20Mapping))
  (for _array_element _output_get
    (Default|Add/RemoveMappingContext _controller_ref true _array_element))
  (Default|Add/RemoveMappingContext _controller_ref false "/Game/Blueprints/Controls/IMC_MenuNavigation.IMC_MenuNavigation")
  (bind _returnvalue (UserInterface|CreateWidget "/Game/Blueprints/GUI/Menu/WBP_PauseMenu.WBP_PauseMenu_C" 0 self))
  (bind _output_get_2 (Variables|Widget|SetPause%20Menu%20ref _returnvalue))
  (UserInterface|Viewport|AddtoViewport _output_get_2 0)
  (Game|SetGamePaused true))

(event Custom|Begin%20Setup%20State
  ;[0 0.1094 0.02125 0.6] Game State
  ;;[0.1079 1 0.9502 0.5] Setup State
  (Default|SwitchSpellBook (Variables|References|GetController%20Ref) false)
  (CallFunction|BLight))

(event Custom|Quit%20Pause%20Menu
  (bind _controller_ref (Variables|References|GetController%20Ref))
  ;[0 0.1094 0.02125 0.6] Game State
  ;;[1 0 0.7648] Pause Menu
  (Widget|RemovefromParent (Variables|Widget|GetPause%20Menu%20ref))
  (for _array_element (Variables|Pause|GetPrevious%20Mapping%20%28Pause%29)
    (Default|Add/RemoveMappingContext _controller_ref false _array_element))
  (Default|Add/RemoveMappingContext _controller_ref true "/Game/Blueprints/Controls/IMC_MenuNavigation.IMC_MenuNavigation")
  (Game|SetGamePaused false))

(event Custom|End%20Setup%20State
  ;[0 0.1094 0.02125 0.6] Game State
  ;;[0.1079 1 0.9502 0.5] Setup State
  ;;;[0.2153 0 1] Fin de la phase et passage à la phase de raid
  (CallFunction|SetGameState "NewEnumerator2"))

(event Custom|End%20Raid%20State
  ;[0 0.1094 0.02125 0.6] Game State
  (CallFunction|SetGameState "NewEnumerator0"))

(event Custom|Begin%20Ritual%20State
  ;[0 0.1094 0.02125 0.6] Game State
  (CallFunction|EndRitualState))

(event Custom|Quit%20Cutscene%20Mode
  ;[0 0.1094 0.02125 0.6] Game State
  ;;[0.08557 0.4948 1] Cutscenes
  (Default|Add/RemoveMappingContext (Variables|References|GetController%20Ref) true "/Game/Blueprints/Controls/IMC_Camera.IMC_Camera"))

(event Custom|Enter%20Cutscene%20Mode
  ;[0 0.1094 0.02125 0.6] Game State
  ;;[0.08557 0.4948 1] Cutscenes
  (Default|Add/RemoveMappingContext (Variables|References|GetController%20Ref) true "/Game/Blueprints/Controls/IMC_Camera.IMC_Camera"))

(event Custom|Activate/Deactivate%20Adventurers
  (params (InputPin :type EMovementMode%20Enum :default "MOVE_None"))
  ;[1 1 1] TEMPORARY
  (Utilities|IsValid (CallFunction|GetWizard) :!label _label
    (:Is%20Valid
      (Utilities|IsValid (CallFunction|GetThief)
        (:Is%20Valid
          (Utilities|IsValid (CallFunction|GetWarrior)
            (:Is%20Valid
              (Development|PrintString "ALL GOOD" true true "(R=0.000000,G=0.660000,B=1.000000,A=1.000000)" 1e+01)
              (Pawn|Components|CharacterMovement|SetMovementMode (Variables|/Script/Engine.Character|GetCharacterMovement (CallFunction|GetWizard)) InputPin 0)
              (Pawn|Components|CharacterMovement|SetMovementMode (Variables|/Script/Engine.Character|GetCharacterMovement (CallFunction|GetThief)) InputPin 0)
              (Pawn|Components|CharacterMovement|SetMovementMode (Variables|/Script/Engine.Character|GetCharacterMovement (CallFunction|GetWarrior)) InputPin 0))
            (:Is%20Not%20Valid
              (Utilities|FlowControl|Delay 0.2 :!label _label_2)
              (goto _label))))
        (:Is%20Not%20Valid
          (goto _label_2))))
    (:Is%20Not%20Valid
      (Development|PrintString "WIZARD AI UNVALID" true true "(R=0.000000,G=0.660000,B=1.000000,A=1.000000)" 2e+01)
      (goto _label_2))))

(event Custom|Use%20Mana
  (params (Amount :type Float%20%28double-precision%29) (IsPreview :type Boolean))
  ;[0 0.04727 1] Mana
  (bind _can_use (CallFunction|TrytoUseMana Amount))
  (if (or _can_use IsPreview)
    (Default|ChangeGauge (Variables|Mana|GetManaGauge) 0.0 true (/ Amount (Variables|Cleanness|GetCleanMultiplyer)) IsPreview)
    (if (not IsPreview)
      (Variables|Mana|SetCan%20Ricover%20Mana true))))

(event Custom|GetChandelierRef
  (params (Chandelier :type BP%20Chandelier%20Object%20Reference))
  ;[1 0.6612 0.3281] Light
  (Utilities|Array|Add (Variables|References|GetChandelier) Chandelier))

(event Custom|GetTorchRef
  (params (Torch :type BP%20Torch%20Object%20Reference))
  ;[1 0.6612 0.3281] Light
  (Utilities|Array|Add (Variables|References|GetTorch) Torch))

(event Custom|GetNbObject
  (for _array_element (Variables|References|GetAllRoomsRef)
    (for _array_element_2 (Variables|/Game/Blueprints/LevelElements/BP_Room.BP_Room_C|GetLinkedPossessables _array_element)
      (Math|Float|IncrementFloat (Variables|Cleanness|GetAllObject)))))

(event Custom|R_Light
  ;[1 0.6612 0.3281] Light
  (for _array_element (Variables|References|GetTorch)
    (Default|SetRedLight _array_element))
  (for _array_element_2 (Variables|References|GetChandelier)
    (Default|SetRedLight _array_element_2)))

(event Custom|HideTrapZone
  ;[1 0.7098 0.1491] HideTrapZone
  (for _array_element (Variables|References|GetAllCoriRef)
    (Utilities|IsValid _array_element
      (:Is%20Valid
        (Default|Hide _array_element)))))

(event Custom|B_Light
  ;[1 0.6612 0.3281] Light
  (for _array_element (Variables|References|GetTorch)
    (Default|SetBlueLight _array_element))
  (for _array_element_2 (Variables|References|GetChandelier)
    (Default|SetBlueLight _array_element_2)))

(event Custom|GetTrapZoneRef
  (params (cori :type BP%20Corridor%20Object%20Reference))
  ;[1 0.7098 0.1491] HideTrapZone
  (Utilities|Array|Add (Variables|References|GetAllCoriRef) cori))

(event Custom|Play%20Track
  (switch Utilities|FlowControl|Switch|SwitchonE_GameState (Variables|GameState|GetE_GameState)
    (:NewEnumerator8
      (Audio|Components|Audio|SetSound (Variables|/Script/Engine.AmbientSound|GetAudioComponent (Variables|Default|GetCurrentTrack)) "/Game/Sounds/Ghost_Tale_-_Title_Screen.Ghost_Tale_-_Title_Screen"))
    (:NewEnumerator1
      (Audio|Components|Audio|SetSound (Variables|/Script/Engine.AmbientSound|GetAudioComponent (Variables|Default|GetCurrentTrack)) "/Game/Sounds/Ghost_Tale_-_Setup.Ghost_Tale_-_Setup"))
    (:NewEnumerator2
      (Audio|Components|Audio|SetSound (Variables|/Script/Engine.AmbientSound|GetAudioComponent (Variables|Default|GetCurrentTrack)) "/Game/Sounds/Ghost_Tale_-_Raid.Ghost_Tale_-_Raid"))))

(event Custom|SetTextTuto
  (bind _main_widget_ref (Variables|Widget|GetMain%20Widget%20Ref))
  (Utilities|FlowControl|Delay 0.2)
  (switch Utilities|FlowControl|Switch|SwitchonE_GameState (Variables|GameState|GetE_GameState)
    (:NewEnumerator1
      (if (Variables|GameState|GetFirstSetup)
        (Variables|GameState|SetFirstSetup false)
        (Default|ActivateTutorial _main_widget_ref "After all this time, I'm finally done cleaning my dungeon !  
I just need to prepare some traps in case some adventurer may have the idea of making a mess into my home. 
I'm sure I have some traps to summon in my cards...")
        (else
          (Default|ActivateTutorial _main_widget_ref "Okay, now I have to set the traps before these morons come back..."))))
    (:NewEnumerator2
      (if (Variables|GameState|GetFirstRaid)
        (Variables|GameState|SetFirstRaid false)
        (Default|ActivateTutorial _main_widget_ref "It's over ! My dungeon is the cleanest dungeon and no one can say anything about it !! 
Hey ! HEY !! It's private property guys !! 
I forgot they can't hear me... 
I'll just scare them away before they make too much of a mess of this place.")
        (else
          (Default|ActivateTutorial _main_widget_ref "When are they gonna stop coming here ! This dungeon isn't for sale !! 
It can't be help, I'll kick them out before they dirty everything in my halls ! ")))))
  (Utilities|FlowControl|Delay 0.1)
  (Default|RemoveTutorial (Variables|Widget|GetMain%20Widget%20Ref)))

(event Custom|Mana%20Ricovery
  (params (Delta%20Time :type Float%20%28double-precision%29))
  (bind _managauge (Variables|Mana|GetManaGauge))
  ;[0 0.04727 1] Mana
  (Default|ChangeGauge _managauge 0.0 false (* Delta%20Time (Variables|Mana|GetReneManaMultiplyer)) false)
  (if (Default|GetIsFull _managauge)
    (Variables|Mana|SetCan%20Ricover%20Mana false)))

(event Custom|Set%20Game%20State
  (params (New%20State :type E_GameState%20Enum :default "NewEnumerator1"))
  ;[0 0.1094 0.02125 0.6] Game State
  ;;[0.3981 0.5104 0.02329] Redéfinit la phase de jeu lance les bons events
  (bind _output_get (Variables|GameState|SetE_GameState New%20State))
  (switch Utilities|FlowControl|Switch|SwitchonE_GameState _output_get
    (:NewEnumerator8
      (CallFunction|PlayTrack :!label _label))
    (:NewEnumerator1
      (CallFunction|BeginSetupState)
      (CallFunction|SetTextTuto :!label _label_2)
      (goto _label))
    (:NewEnumerator2
      (CallFunction|BeginRaidState)
      (goto _label_2))
    (:NewEnumerator0
      (CallFunction|BeginRitualState))
    (:NewEnumerator6
      (CallFunction|OpenPauseMenu (Default|GetActiveMapping (Variables|References|GetController%20Ref))))))

(event Custom|Make%20Dirt
  (params (Dirt%20Amount :type Float%20%28double-precision%29))
  (bind _cleannessgauge (Variables|Cleanness|GetCleannessGauge))
  ;[1 0.9252 0 0.3] Cleanness
  ;;[1 0.2309 0 0.5] Les aventuriers mettent le bazar
  (Default|ChangeGauge _cleannessgauge 0.0 true Dirt%20Amount false)
  ;;[1 0.7404 0 0.5] On met à jour notre bonus de propreté
  (Variables|Cleanness|SetCleanMultiplyer (CallFunction|SetCleanMutiplyer (Default|GetCurrentStep _cleannessgauge))))

(event Custom|Tidy%20Up
  (params (Cleanness%20Amount :type Float%20%28double-precision%29))
  (bind _cleannessgauge (Variables|Cleanness|GetCleannessGauge))
  ;[1 0.9252 0 0.3] Cleanness
  ;;[0.6984 1 0 0.5] On range
  (Default|ChangeGauge _cleannessgauge 0.0 false Cleanness%20Amount false)
  ;;[1 0.7404 0 0.5] On met à jour notre bonus de propreté
  (Variables|Cleanness|SetCleanMultiplyer (CallFunction|SetCleanMutiplyer (Default|GetCurrentStep _cleannessgauge))))

(event Custom|Start%20Timer
  ;[0.122 1 0.1198 0.5] Timer
  ;;[0 0.3854 0.08175] Reparamètre les données et lance le timer
  (Variables|Timer|SetMin%20Timer (Variables|Timer|GetReset%20Timer))
  (Variables|Timer|SetSec%20Timer 0)
  (CallFunction|Timer))

(event Custom|Timer
  ;[0.122 1 0.1198 0.5] Timer
  ;;[0 0.6667 0.5848] Vérifie si le timer est fini
  (if (and (== (Variables|Timer|GetSec%20Timer) 0) (== (Variables|Timer|GetMin%20Timer) 0))
    ;;[0.0158 0.3558 0.6042] Lance le changement d'étape
    (Widget|RemovefromParent (Variables|Widget|GetTimer%20Widget%20Ref))
    (CallFunction|EndSetupState)
    (else
      ;;[0.0153 1 0] Timer.
      ;; Reboucle sur lui-même tant que les deux valeurs ne sont pas à zéro
      (if (== (Variables|Timer|GetSec%20Timer) 0)
        (Variables|Timer|SetSec%20Timer 59)
        (Math|Integer|DecrementInt (Variables|Timer|GetMin%20Timer)
          (:%20%20
            _))
        (else
          (Math|Integer|DecrementInt (Variables|Timer|GetSec%20Timer)
            (:%20%20
              _))))
      (Utilities|FlowControl|Delay 1.0)
      (CallFunction|Timer))))

(event Custom|End%20Ritual%20State
  ;[0 0.1094 0.02125 0.6] Game State
  (CallFunction|SetGameState "NewEnumerator3"))

(event EventBeginPlay
  (bind _managauge (Variables|Mana|GetManaGauge))
  (bind _cleannessgauge (Variables|Cleanness|GetCleannessGauge))
  ;[1 1 1] Event Begin Play
  (bind _returnvalue (Actor|GetActorOfClass "/Script/Engine.AmbientSound"))
  (Variables|Default|SetCurrentTrack _returnvalue)
  (Default|ChangeGauge _managauge 0.0 false (Default|GetMaxGauge _managauge) false)
  (Default|ChangeGauge _cleannessgauge 0.0 false (Default|GetMaxGauge _cleannessgauge) false)
  (Utilities|FlowControl|Delay 0.1)
  (CallFunction|GetNbObject)
  (bind _asbp_camera_controller (Utilities|Casting|CastToBP_CameraController (Game|GetPlayerController 0)))
  (Variables|References|SetController%20Ref _asbp_camera_controller)
  (CallFunction|PlayTrack)
  (CallFunction|SetGameState (Variables|GameState|GetE_GameState)))

(event EventTick
  (params (DeltaSeconds :type Float%20%28single-precision%29))
  ;[1 0.9437 0] Event Tick
  (if (Variables|Mana|GetCan%20Ricover%20Mana)
    (CallFunction|ManaRicovery DeltaSeconds)))

(fn ConstructionScript)

(fn AddDoor
  (params (Door :type BP%20Door%20Object%20Reference))
  (Utilities|Array|Add (Variables|References|GetAllDoorsRef) Door))

(fn AddRoom
  (params (Room :type BP%20Room%20Object%20Reference))
  (Utilities|Array|Add (Variables|References|GetAllRoomsRef) Room))

(fn AddThief
  (params (Thief :type BP%20Thief%20Object%20Reference))
  (Variables|References|SetThief%20Ref Thief))

(fn AddWizard
  (params (Wizard :type BP%20Wizard%20Object%20Reference))
  (Variables|References|SetWizard%20Ref Wizard))

(fn AddWarrior
  (params (Warrior :type BP%20Warrior%20Object%20Reference))
  (Variables|References|SetWarrior%20Ref Warrior))

(fn GetThief
  (return (Variables|References|GetThief%20Ref)))

(fn GetWizard
  (return (Variables|References|GetWizard%20Ref)))

(fn GetWarrior
  (return (Variables|References|GetWarrior%20Ref)))

(fn TrytoUseMana
  (params (Amont :type Float%20%28double-precision%29))
  (bind _output_get (Variables|Mana|SetCan%20Use%20Mana (not (< (- (Default|GetCurrentGauge (Variables|Mana|GetManaGauge)) Amont) 0.0))))
  (return _output_get))

(fn GetManaPercent
  (params (IsPreview :type Boolean))
  (return (Default|GetGaugePercent (Variables|Mana|GetManaGauge) IsPreview 1e+02)))

(fn GetCleannessPercent
  (return (Default|GetGaugePercent (Variables|Cleanness|GetCleannessGauge) false (Variables|Cleanness|GetAllObject))))

(fn SetCleanMutiplyer
  (params (Clean%20Level :type Integer))
  (bind _cleanlevelmultiplyer (Variables|Cleanness|GetCleanLevelMultiplyer))
  (bind (_value _returnvalue) (Utilities|Map|Find _cleanlevelmultiplyer Clean%20Level))
  (if _returnvalue
    (return _value)
    (else
      (return 1.0))))

(fn SetMainWidget
  (params (Widget :type WBP%20Main%20Object%20Reference))
  (Variables|Widget|SetMain%20Widget%20Ref Widget))

(fn GetTimer
  (return (Variables|Timer|GetMin%20Timer) (Variables|Timer|GetSec%20Timer) (Variables|Timer|GetReset%20Timer)))